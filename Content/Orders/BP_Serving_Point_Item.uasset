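; Serving point that gives visual feedback when the player delivers dishes for orders.
; Each Tick it highlights and outlines its mesh while the player holds a frying, fishing or soup dish, otherwise restoring the default look.
; ChangeToGreen and ChangeToRed show correct or wrong order materials, pausing that check briefly.
; A wrong order also raises then lowers a stop sign, spawned on BeginPlay near BP_ServingPlace, with a guard against retriggering.
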(event `self.ReceiveTick`
  (params (DeltaSeconds :type "Float (single-precision)"))
  (bind _staticmeshcomponent (`self.StaticMeshComponent`))
  (if (`self.Served`)
    (if (> (`self.ServedTime`) 1.5)
      (set `self.Served` false)
      (else
        (set `self.ServedTime` (+ (`self.ServedTime`) DeltaSeconds))))
    (else
      (bind _returnvalue (`GameplayStatics.GetActorOfClass` "/Game/ThirdPerson/Blueprints/BP_ThirdPersonCharacter.BP_ThirdPersonCharacter_C"))
      (if (`/Game/ThirdPerson/Blueprints/BP_ThirdPersonCharacter.HasItem` _returnvalue)
        (bind _returnvalue_2 (`GameplayStatics.GetObjectClass` (`/Game/ThirdPerson/Blueprints/BP_ThirdPersonCharacter.ItemReference` _returnvalue)))
        (if (`KismetMathLibrary.ClassIsChildOf` _returnvalue_2 "/Game/FinalDish/BP_FryingDish.BP_FryingDish_C")
          (`PrimitiveComponent.SetMaterial` _staticmeshcomponent 0 "/Game/Material/M_Serving_Highlight2.M_Serving_Highlight2" :!label _label)
          (`MeshComponent.SetOverlayMaterial` _staticmeshcomponent "/Game/Material/M_Serving_Outline.M_Serving_Outline")
          (elif (`KismetMathLibrary.ClassIsChildOf` _returnvalue_2 "/Game/FinalDish/BP_FishingDish.BP_FishingDish_C")
            (goto _label)
            (elif (`KismetMathLibrary.ClassIsChildOf` _returnvalue_2 "/Game/FinalDish/BP_SoupDish.BP_SoupDish_C")
              (goto _label)
              (else
                (`PrimitiveComponent.SetMaterial` _staticmeshcomponent 0 "/Game/LevelPrototyping/AssetPacks/KayKit_Restaurant_Bits/fbx/restaurant.restaurant" :!label _label_2)
                (`MeshComponent.SetOverlayMaterial` _staticmeshcomponent "/Game/Material/M_Blank.M_Blank")))))
        (else
          (goto _label_2))))))

(event `ChangeToGreen`
  (bind _staticmeshcomponent (`self.StaticMeshComponent`))
  ;[1 1 1] If an order for the final dish is found
  (`PrimitiveComponent.SetMaterial` _staticmeshcomponent 0 "/Game/Material/M_Serving_Highlight_Correct.M_Serving_Highlight_Correct")
  (`MeshComponent.SetOverlayMaterial` _staticmeshcomponent "/Game/Material/M_Wire_Outline_Fixed.M_Wire_Outline_Fixed")
  (set `self.Served` true :!label _label_3)
  (set `self.ServedTime` 0.0))

(event `ChangeToRed`
  (bind _staticmeshcomponent (`self.StaticMeshComponent`))
  ;[1 1 1] If an order for the final dish is not found
  (`PrimitiveComponent.SetMaterial` _staticmeshcomponent 0 "/Game/Material/M_Serving_Highlight_Wrong.M_Serving_Highlight_Wrong")
  (`MeshComponent.SetOverlayMaterial` _staticmeshcomponent "/Game/Material/M_Wire_Outline_Broken.M_Wire_Outline_Broken")
  (`|ExecutionSequence`
    (:`then_0`
      (goto _label_3))
    (:`then_1`
      (if (not (`self.Lerping`))
        (set `self.Lerping` true)
        (`/Game/FinalDish/BP_StopSign.LerpSignUp` (`self.StopSign`))
        (`KismetSystemLibrary.Delay` 1.2)
        (`/Game/FinalDish/BP_StopSign.LerpSignDown` (`self.StopSign`))
        (set `self.Lerping` false)))))

(event `self.ReceiveBeginPlay`
  (bind _returnvalue (`GameplayStatics.GetActorOfClass` "/Game/FinalDish/BP_ServingPlace.BP_ServingPlace_C"))
  (bind (_returnvalue_location _returnvalue_rotation) (`KismetMathLibrary.BreakTransform` (`self.GetTransform` _returnvalue)))
  (bind _returnvalue_2 (`|SpawnActorFromClass` "/Game/FinalDish/BP_StopSign.BP_StopSign_C" (`KismetMathLibrary.MakeTransform` (- _returnvalue_location (-135.0 135.0 350.0)) _returnvalue_rotation) "Undefined" "MultiplyWithRoot" null null))
  (set `self.StopSign` _returnvalue_2))

(fn `UserConstructionScript`)
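; Player character component that shows orders from the level's BP_OrderManager as on-screen widgets.
; On BeginPlay it finds the manager and binds to its create-order event.
; Each event adds a UI_OrderGui to the owning player's screen, copying name and texture from the supplied order GUI.
; The new widget is passed back to the order as its screen GUI reference.
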(event `self.ReceiveBeginPlay`
  (bind _asbp_third_person_character (cast `/Game/ThirdPerson/Blueprints/BP_ThirdPersonCharacter` (`self.GetOwner`)))
  (set `self.Owner` _asbp_third_person_character)
  (bind _returnvalue (`GameplayStatics.GetActorOfClass` "/Game/Orders/BP_OrderManager.BP_OrderManager_C"))
  (bind _output_get (set `self.OrderManager` _returnvalue))
  (add `/Game/Orders/BP_OrderManager.CreateOrderGuiInScreen` _output_get (delegate `CreateOrderOnScreen`)))

(event `CreateOrderOnScreen`
  (params (OrderGuiRefrence :type "/Game/Orders/UI_OrderGui Object Reference") (OrderRefrence :type "/Game/Orders/BP_Order Object Reference"))
  (bind _asplayer_controller (cast `PlayerController` (`Pawn.GetController` (`self.Owner`))))
  (bind _output_get (set `self.Controller` _asplayer_controller))
  (bind _returnvalue (`|CreateWidget` "/Game/Orders/UI_OrderGui.UI_OrderGui_C" _output_get))
  (`UserWidget.AddToPlayerScreen` _returnvalue 0)
  (`/Game/Orders/UI_OrderGui.SetUpScreenVersion` _returnvalue (`/Game/Orders/UI_OrderGui.TempName` OrderGuiRefrence) (`/Game/Orders/UI_OrderGui.TempTexture` OrderGuiRefrence))
  (`/Game/Orders/BP_Order.SetScreenGuiRefrence` OrderRefrence _returnvalue))

(event `self.ReceiveTick`
  (params (DeltaSeconds :type "Float (single-precision)")))
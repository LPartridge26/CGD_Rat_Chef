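; BP_Order is a timed order actor that shows its elapsed-time progress on a UI_OrderGui widget, which it initializes with itself through SetUpGui.
; Tick advances the timer and, past DeleteTime, destroys the actor and notifies the BP_OrderManager found by the OrderSpace tag.
; LerpOrder uses a timeline to slide the order along Y when another is deleted, blending from its current transform each update.
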(event `self.ReceiveBeginPlay`)

(event `self.ReceiveTick`
  (params (DeltaSeconds :type "Float (single-precision)"))
  (bind _output_get (set `self.CurrentTime` (+ DeltaSeconds (`self.CurrentTime`))))
  (if (> _output_get (`self.DeleteTime`))
    (`self.K2_DestroyActor`)
    (bind _outactors (`GameplayStatics.GetAllActorsWithTag` "OrderSpace"))
    (for _array_element _outactors
      (bind _asbp_order_manager (cast `/Game/Orders/BP_OrderManager` _array_element))
      (`/Game/Orders/BP_OrderManager.OrderDeleted` _asbp_order_manager self)
      (`KismetSystemLibrary.PrintString` "Hello"))
    (else
      (bind _asui_order_gui (cast `/Game/Orders/UI_OrderGui` (`WidgetComponent.GetUserWidgetObject` (`self.Widget`))))
      (`/Game/Orders/UI_OrderGui.SetThePercentage` _asui_order_gui (/ (`self.CurrentTime`) (`self.DeleteTime`))))))

(event `SetUpGui`
  ;[1 1 1] Set up the Gui
  (bind _asui_order_gui (cast `/Game/Orders/UI_OrderGui` (`WidgetComponent.GetUserWidgetObject` (`self.Widget`))))
  (`/Game/Orders/UI_OrderGui.SetUpGui` _asui_order_gui self))

(event `LerpOrder`
  (params (OrderDistance :type Integer))
  (bind (_returnvalue_location _returnvalue_rotation _returnvalue_scale) (`KismetMathLibrary.BreakTransform` (`self.GetTransform` self)))
  ;[1 1 1] Lerp the rest of the orders as one has just been deleted
  (set `self.LerpTransform` (`KismetMathLibrary.MakeTransform` (`KismetMathLibrary.MakeVector` (.x _returnvalue_location) (+ (.y _returnvalue_location) OrderDistance) (.z _returnvalue_location)) _returnvalue_rotation _returnvalue_scale))
  (bind (_direction _alpha) (`Timeline|OrderLerp`)
    (:`Update`
      (`self.K2_SetActorTransform` self (`KismetMathLibrary.TLerp` (`self.GetTransform` self) (`self.LerpTransform`) _alpha) false false))
    (:`Finished`
      (`TimelineComponent.SetNewTime` (`self.OrderLerp`) 0.0))))

(fn `UserConstructionScript`)
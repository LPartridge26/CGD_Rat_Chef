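; Physics object that can be pushed until it falls, then smashes on the floor or splats a non-rat (chef) player with a timed screen overlay.
; A state switch drives it: Tick flags Pushable as Falling on Y-axis speed, and overlaps while Falling trigger the hit.
; Smashing plays FX, hides the actor as Inactive, then resets it to its start transform after a delay.
; Several splat-check and UI functions are empty stubs.
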(event `SplatOverlayTimer`
  (`KismetSystemLibrary.Delay` (`self.Splat Time`))
  (`self.Remove Splat UI`))

(event `Smash`
  (bind _returnvalue (`NiagaraFunctionLibrary.SpawnSystemAttached` "/Game/PhysicsObjects/FX_Smash.FX_Smash" (`self.StaticMesh`) "None" (0.0 0.0 0.0) (struct) "KeepRelativeOffset"))
  (`KismetSystemLibrary.Delay` 0.2)
  (`ActorComponent.K2_DestroyComponent` _returnvalue)
  (`self.Inactive`))

(event `Inactive`
  (set `self.States` "NewEnumerator3")
  (`self.SetActorHiddenInGame` true)
  (`KismetSystemLibrary.Delay` (`self.Inactive Time`))
  (`self.Set Active`))

(event `self.ReceiveBeginPlay`
  (set `self.States` "NewEnumerator0")
  (set `self.Start Transform` (`self.GetTransform`))
  (bind _outactors (`GameplayStatics.GetAllActorsOfClass` "/Game/Managers/BP_ScoreManager.BP_ScoreManager_C"))
  (set `self.Score Manager` (`|GetArrayItem` _outactors)))

(event `self.ReceiveTick`
  (params (DeltaSeconds :type "Float (single-precision)"))
  (switch `/Game/PhysicsObjects/PhysicsObjectStates` (`self.States`)
    (:`NewEnumerator0`
      (`self.Check Velocity`))))

(event `self.ReceiveActorBeginOverlap`
  (params (OtherActor :type "Actor Object Reference"))
  (switch `/Game/PhysicsObjects/PhysicsObjectStates` (`self.States`)
    (:`NewEnumerator1`
      (bind _asbp_third_person_character (cast `/Game/ThirdPerson/Blueprints/BP_ThirdPersonCharacter` OtherActor)
        (:`then`
          (if (not (`/Game/ThirdPerson/Blueprints/BP_BaseCharacter.IsRat` _asbp_third_person_character))
            (`self.Hit Chef ` _asbp_third_person_character)))
        (:`CastFailed`
          (`self.Hit Floor`))))))

(fn `Check for Chef `
  (locals (NewLocalVar :type "HitResult Structure")))

(fn `Check Velocity`
  (bind (_returnvalue_x _returnvalue_y) (`KismetMathLibrary.BreakVector` (`self.GetVelocity`)))
  (if (or (< _returnvalue_y -50.0) (> _returnvalue_y 50.0))
    (`KismetSystemLibrary.PrintString` "Changing to falling")
    (set `self.States` "NewEnumerator1")))

(fn `Create Chef Splat UI`)

(fn `Hit Chef `
  (params (Chef :type "/Game/ThirdPerson/Blueprints/BP_ThirdPersonCharacter Object Reference"))
  (`self.Smash`)
  (`/Game/ThirdPerson/Blueprints/BP_ThirdPersonCharacter.Add Splat Overlay` Chef (`self.Splat Time`))
  (`GameplayStatics.PlaySound2D` (`self.Hit Sound`) 1.0 1.0 0.0 null null))

(fn `Hit Floor`
  (`GameplayStatics.PlaySound2D` (`self.Smashed Sound`) 1.0 1.0 0.0 null null)
  (`self.Smash`))

(fn `Remove Splat UI`
  (bind _splat_widget (`self.Splat Widget`)
    (:`then`
      (`Widget.RemoveFromParent` _splat_widget)
      (set `self.Splat Widget` null))
    (:`else`)))

(fn `Set Active`
  (set `self.States` "NewEnumerator0")
  (`self.K2_SetActorTransform` (`self.Start Transform`))
  (`self.SetActorHiddenInGame` false))

(fn `Splat checks`)

(fn `UserConstructionScript`)
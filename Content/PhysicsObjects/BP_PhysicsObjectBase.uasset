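; Base physics object actor that cycles through Pushable, Falling and Inactive states.
; Tick switches it to Falling when Y velocity drops below a threshold.
; Overlapping a non-rat third-person character hides it, then restores its start transform after a delay; this overlap switches on a literal Falling, not the current state.
; The chef and splat checks are empty stubs.
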(event `Inactive`
  (set `self.States` "NewEnumerator3")
  (`self.SetActorHiddenInGame` true)
  (`KismetSystemLibrary.Delay` (`self.Inactive Time`))
  (`self.Set Active`))

(event `self.ReceiveBeginPlay`
  (set `self.States` "NewEnumerator0")
  (set `self.Start Transform` (`self.GetTransform`)))

(event `self.ReceiveTick`
  (params (DeltaSeconds :type "Float (single-precision)"))
  (switch `/Game/PhysicsObjects/PhysicsObjectStates` (`self.States`)
    (:`NewEnumerator0`
      (`self.Check Velocity`))
    (:`NewEnumerator1`
      (`self.Check for Chef `))))

(event `self.ReceiveActorBeginOverlap`
  (params (OtherActor :type "Actor Object Reference"))
  (switch `/Game/PhysicsObjects/PhysicsObjectStates` "NewEnumerator1"
    (:`NewEnumerator1`
      (bind _asbp_third_person_character (cast `/Game/ThirdPerson/Blueprints/BP_ThirdPersonCharacter` OtherActor))
      (if (not (`/Game/ThirdPerson/Blueprints/BP_BaseCharacter.IsRat` _asbp_third_person_character))
        (`self.Inactive`)))))

(fn `Check for Chef `
  (locals (NewLocalVar :type "HitResult Structure")))

(fn `Check Velocity`
  (bind (_returnvalue_x _returnvalue_y) (`KismetMathLibrary.BreakVector` (`self.GetVelocity`)))
  (if (< _returnvalue_y -1.0)
    (`KismetSystemLibrary.PrintString` "Hello")
    (set `self.States` "NewEnumerator1")))

(fn `Set Active`
  (set `self.States` "NewEnumerator0")
  (`self.K2_SetActorTransform` (`self.Start Transform`))
  (`self.SetActorHiddenInGame` false))

(fn `Splat checks`)

(fn `UserConstructionScript`)
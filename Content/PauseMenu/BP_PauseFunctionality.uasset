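; BP_PauseFunctionality toggles game pause from the IA_Pause Enhanced Input action.
; On BeginPlay it caches the first BP_TemporaryPauseObject found in the level.
; Each press flips the paused state and notifies that object through OnPausePressed when pausing or OnContinuePressed when resuming.
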(event `self.ReceiveBeginPlay`
  (bind _outactors (`GameplayStatics.GetAllActorsOfClass` "/Game/PauseMenu/BP_TemporaryPauseObject.BP_TemporaryPauseObject_C"))
  (set `self.NewVar` (`|GetArrayItem` _outactors)))

(event `EnhancedInput|/Game/ThirdPerson/Input/Default_Actions/IA_Pause`
  (params (ActionValue :type "Vector2D Structure") (ElapsedSeconds :type "Float (double-precision)") (TriggeredSeconds :type "Float (double-precision)") (InputAction :type "InputAction Object Reference" :default "/Game/ThirdPerson/Input/Default_Actions/IA_Pause.IA_Pause"))
  (:`Started`
    (if (`GameplayStatics.IsGamePaused`)
      (`GameplayStatics.SetGamePaused` false)
      (`/Game/PauseMenu/BP_TemporaryPauseObject.On Continue Pressed` (`self.NewVar`))
      (else
        (`GameplayStatics.SetGamePaused` true)
        (`/Game/PauseMenu/BP_TemporaryPauseObject.On Pause Pressed` (`self.NewVar`))))))
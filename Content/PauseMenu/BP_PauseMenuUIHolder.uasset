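; Actor that manages the pause menu: it creates or removes the UI_PauseMenu widget while toggling game pause and mouse cursor.
; Continue restores the previous input on every BP_BaseCharacter, while Quit opens MainMenuMap.
; Button navigation steps a wrapping index through an array of the widget's buttons, faking hover by swapping style brushes.
; Accept picks Continue or Quit by the hovered button's object name.
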(fn `AcceptButton`
  (`self.Button Hovered`
    (:`then`
      (if (`KismetStringLibrary.EqualEqual_StrStr` (`KismetSystemLibrary.GetObjectName` (`self.Button Hovered`)) "ContinueButton")
        (`self.On Continue Pressed`)
        (else
          (`self.On Quit Pressed `))))
    (:`else`)))

(fn `Check Index`
  (params (Index :type Integer))
  (locals (`Index L` :type Integer))
  (bind _output_get (set `local.Index L` Index))
  (if (>= _output_get (`KismetArrayLibrary.Array_Length` (`self.Buttons Array `)))
    (set `self.Button Index` 0)
    (elif (< (`local.Index L`) 0)
      (set `self.Button Index` (- (`KismetArrayLibrary.Array_Length` (`self.Buttons Array `)) 1))
      (else
        (set `self.Button Index` (`local.Index L`))))))

(fn `Create UI`
  (bind _returnvalue (`|CreateWidget` "/Game/PauseMenu/UI_PauseMenu.UI_PauseMenu_C"))
  (bind _output_get (set `self.Pause Menu UI` _returnvalue))
  (`UserWidget.AddToViewport` _output_get 0)
  (`self.Set button array`))

(fn `Destroy UI`
  (`KismetArrayLibrary.Array_Clear` (`self.Buttons Array `))
  (`Widget.RemoveFromParent` (`self.Pause Menu UI`))
  (set `self.Pause Menu UI` null))

(fn `On Continue Pressed`
  (set `PlayerController.bShowMouseCursor` false (`GameplayStatics.GetPlayerController` 0))
  (`self.Destroy UI`)
  (bind _outactors (`GameplayStatics.GetAllActorsOfClass` "/Game/ThirdPerson/Blueprints/BP_BaseCharacter.BP_BaseCharacter_C"))
  (for _array_element _outactors
    (`/Game/ThirdPerson/Blueprints/BP_BaseCharacter.SwitchMenuTo_PreviousInput` _array_element))
  (`GameplayStatics.SetGamePaused` false))

(fn `On Pause Pressed`
  (set `PlayerController.bShowMouseCursor` true (`GameplayStatics.GetPlayerController` 0))
  (`self.Create UI`)
  (`GameplayStatics.SetGamePaused` true))

(fn `On Quit Pressed `
  (`GameplayStatics.OpenLevel` "MainMenuMap"))

(fn `Set button array`
  (bind _continuebutton (`/Game/PauseMenu/UI_PauseMenu.ContinueButton` (`self.Pause Menu UI`)))
  (bind _quitbutton (`/Game/PauseMenu/UI_PauseMenu.QuitButton` (`self.Pause Menu UI`)))
  (set `Button.WidgetStyle` (`self.Menu Button Style`) _continuebutton)
  (`KismetArrayLibrary.Array_Add` (`self.Buttons Array `) _continuebutton)
  (set `Button.WidgetStyle` (`self.Menu Button Style`) _quitbutton)
  (`KismetArrayLibrary.Array_Add` (`self.Buttons Array `) _quitbutton)
  (`self.Update Button Hovered` 1)
  (set `self.Button Hovered` (`/Game/PauseMenu/UI_PauseMenu.ContinueButton` (`self.Pause Menu UI`))))

(fn `Update Button Hovered`
  (params (Input :type Integer))
  (locals (`Button To Hover L` :type "Button Object Reference"))
  (bind (_menu_button_style_normal _menu_button_style_hovered) (break `ButtonStyle` (`self.Menu Button Style`)))
  (bind _menu_button_style_normal_2 (break `ButtonStyle` (`self.Menu Button Style`)))
  (`self.Check Index` (+ Input (`self.Button Index`)))
  (bind _output_get (set `local.Button To Hover L` (`|GetArrayItem` (`self.Buttons Array `) (`self.Button Index`))))
  (set `Button.WidgetStyle` (make `ButtonStyle` _menu_button_style_hovered) _output_get)
  (bind _button_hovered (`self.Button Hovered`)
    (:`then`
      (set `Button.WidgetStyle` (make `ButtonStyle` _menu_button_style_normal_2) _button_hovered)
      (set `self.Button Hovered` (`local.Button To Hover L`)))
    (:`else`)))

(fn `UserConstructionScript`)
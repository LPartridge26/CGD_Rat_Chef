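; Temporary actor that manages the pause menu: it creates and tears down the UI_PauseMenu widget and toggles the game's paused state.
; Pausing shows the mouse cursor, adds the widget to the viewport and pauses the game; continuing reverses all three.
; Quitting opens the main menu map by name.
; The pause, continue and quit functions have no callers here, as the event graph is empty.
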(fn `Create UI`
  (bind _returnvalue (`|CreateWidget` "/Game/PauseMenu/UI_PauseMenu.UI_PauseMenu_C"))
  (bind _output_get (set `self.Pause Menu UI` _returnvalue))
  (`UserWidget.AddToViewport` _output_get 0))

(fn `Destroy UI`
  (`Widget.RemoveFromParent` (`self.Pause Menu UI`))
  (set `self.Pause Menu UI` null))

(fn `On Continue Pressed`
  (set `PlayerController.bShowMouseCursor` false (`GameplayStatics.GetPlayerController` 0))
  (`self.Destroy UI`)
  (`GameplayStatics.SetGamePaused` false))

(fn `On Pause Pressed`
  (set `PlayerController.bShowMouseCursor` true (`GameplayStatics.GetPlayerController` 0))
  (`self.Create UI`)
  (`GameplayStatics.SetGamePaused` true))

(fn `On Quit Pressed `
  (`GameplayStatics.OpenLevel` "MainMenuMap"))

(fn `UserConstructionScript`)
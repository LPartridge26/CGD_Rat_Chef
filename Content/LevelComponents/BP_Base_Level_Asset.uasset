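; BP_Base_Level_Asset is a base level prop actor that can turn see-through while the rat character overlaps it.
; When its Transparent flag is set, begin overlap with BP_RatCharacter swaps the StaticMesh's first material slot to M_Transparent.
; End overlap sets that slot to the fixed Restaurant material rather than restoring a cached original.
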(event `self.ReceiveActorBeginOverlap`
  (params (OtherActor :type "Actor Object Reference"))
  (cast `/Game/ThirdPerson/Blueprints/BP_RatCharacter` OtherActor)
  (if (`self.Transparent`)
    (`PrimitiveComponent.SetMaterial` (`self.StaticMesh`) 0 "/Game/Material/M_Transparent.M_Transparent")))

(event `self.ReceiveActorEndOverlap`
  (params (OtherActor :type "Actor Object Reference"))
  (cast `/Game/ThirdPerson/Blueprints/BP_RatCharacter` OtherActor)
  (if (`self.Transparent`)
    (`PrimitiveComponent.SetMaterial` (`self.StaticMesh`) 0 "/Game/LevelPrototyping/AssetPacks/KayKit_Restaurant_Bits/fbx/restaurant.restaurant")))

(fn `UserConstructionScript`)
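; Manager Blueprint that shows an on-screen score popup for a chef player when they complete a minigame or serve a meal.
; Each trigger removes any existing popup, then creates a UI_Chef_ScreenScoreEffect widget on the screen of ChefActor's local viewing player.
; Setting manager values stores the chef and clears RoundEnded, while round reset sets it.
; RoundEnded blocks only the minigame popup, as serving a meal bypasses that check.
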(event `/Game/PlayerEventsBPI/BPI_ChefEvents.Chef_SetManagerValues`
  (params (ChefActor :type "/Game/ThirdPerson/Blueprints/BP_ThirdPersonCharacter Object Reference"))
  ;[0 0.1294 1 1 35] SetManagerValues
  (set `self.ChefActor` ChefActor)
  (set `self.RoundEnded` false))

(event `/Game/PlayerEventsBPI/BPI_ChefEvents.Chef_RoundReset`
  ;[0 0.1294 1 1 35] RoundReset
  (set `self.RoundEnded` true))

(event `/Game/PlayerEventsBPI/BPI_ChefEvents.Chef_CompletedMinigame`
  ;[0 0.1294 1 1 35] Create Score Effect
  (if (not (`self.RoundEnded`))
    (if (`KismetSystemLibrary.IsValid` (`self.NewScorePopup`)) :!label _label
      (`Widget.RemoveFromParent` (`self.NewScorePopup`)))
    (`self.CreateScoreEffect`)))

(event `/Game/PlayerEventsBPI/BPI_ChefEvents.Chef_ServedMeal`
  ;[0 0.1294 1 1 35] Create Score Effect
  (goto _label))

(fn `CreateScoreEffect`
  (bind _returnvalue (`|CreateWidget` "/Game/ScoreUI/UI_Chef_ScreenScoreEffect.UI_Chef_ScreenScoreEffect_C" (`Pawn.GetLocalViewingPlayerController` (`self.ChefActor`))))
  (bind _output_get (set `self.NewScorePopup` _returnvalue))
  (`UserWidget.AddToPlayerScreen` _output_get 0))

(fn `UserConstructionScript`)
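; Rat score-effect manager that shows a screen score popup for a rat's player when that rat finishes a minigame.
; It stores the rat reference and a round-ended flag, set on setup and round reset, and ignores minigame endings once the round is over.
; Each ending removes the previous popup and creates a new UI_Rat_ScreenScoreEffect widget on that player's screen.
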(event `/Game/PlayerEventsBPI/BPI_RatEvents.Rat_SetManagerValues`
  (params (RatActor :type "/Game/ThirdPerson/Blueprints/BP_RatCharacter Object Reference"))
  ;[0 0.1294 1 1 35] SetManagerValues
  (set `self.Rat Actor` RatActor)
  (set `self.RoundEnded` false))

(event `/Game/PlayerEventsBPI/BPI_RatEvents.Rat_RoundReset`
  ;[0 0.1294 1 1 35] RoundReset
  (set `self.RoundEnded` true))

(event `/Game/PlayerEventsBPI/BPI_RatEvents.Rat_EndedMinigame`
  ;[0 0.1294 1 1 35] Create Score Effect
  (if (not (`self.RoundEnded`))
    (if (`KismetSystemLibrary.IsValid` (`self.NewScorePopup`))
      (`Widget.RemoveFromParent` (`self.NewScorePopup`)))
    (`self.CreateScoreEffect`)))

(fn `CreateScoreEffect`
  (bind _returnvalue (`|CreateWidget` "/Game/ScoreUI/UI_Rat_ScreenScoreEffect.UI_Rat_ScreenScoreEffect_C" (`Pawn.GetLocalViewingPlayerController` (`self.Rat Actor`))))
  (bind _output_get (set `self.NewScorePopup` _returnvalue))
  (`UserWidget.AddToPlayerScreen` _output_get 0))

(fn `UserConstructionScript`)
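; Manager Blueprint that shows and hides guide markers to steer the chef through each stage of preparing and serving an order.
; Setup caches Chef, Rat and all BPI_GuideMarkerHolder actors, showing only ingredient markers.
; GuideMarkerCheck assigns marker owners by actor string, then toggles non-rat markers by LastAction and marker type.
; After ingredient pickup, the lowest-timed order's GUI texture picks the Blacksmith, Fishing or Mixing station marker.
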(event `Set GuideMarker Values`
  (bind _roundmanager (`self.RoundManager`))
  ;[0 0.1291 1 1 35] SetManagerValues
  (set `self.ChefActor` (`/Game/Managers/BP_RoundManager.Chef` _roundmanager))
  (set `self.RatActor` (`/Game/Managers/BP_RoundManager.Rat` _roundmanager))
  (bind _outactors (`GameplayStatics.GetAllActorsWithInterface` "/Game/GuideMarkerGUI/BPI_GuideMarkerHolder.BPI_GuideMarkerHolder_C"))
  (set `self.GuideMarkers` _outactors)
  (set `self.LastAction` "Started")
  (`self.SetMarkerDisplays`))

(event `SetMarkerDisplays`
  ;[0 0.1291 1 1 35] SetMarkerDisplays
  (for _array_element (`self.GuideMarkers`)
    (bind _markertype (message `/Game/GuideMarkerGUI/BPI_GuideMarkerHolder.GetMarkerType` _array_element))
    (if (`KismetStringLibrary.EqualEqual_StrStr` _markertype "Ingredient")
      (message `/Game/GuideMarkerGUI/BPI_GuideMarkerHolder.DisplayMarker` _array_element)
      (else
        (message `/Game/GuideMarkerGUI/BPI_GuideMarkerHolder.HideMarker` _array_element)))))

(event `GuideMarkerCheck`
  ;[0.2292 0.358 1 1 35] GuideMarkerCheck
  (for _array_element (`self.GuideMarkers`)
    (bind _actorname (message `/Game/GuideMarkerGUI/BPI_GuideMarkerHolder.Marker_GetActorString` _array_element))
    (if (`KismetStringLibrary.EqualEqual_StrStr` _actorname "Chef")
      (`self.MarkerDisplayCheck` _array_element (`self.ChefActor`))
      (elif (`KismetStringLibrary.EqualEqual_StrStr` _actorname "Rat")
        (`self.MarkerDisplayCheck` _array_element (`self.RatActor`))
        (elif (`KismetStringLibrary.EqualEqual_StrStr` _actorname "Both")
          (`self.MarkerDisplayCheck` _array_element (`self.ChefActor`) (`self.RatActor`)))))))

(fn `ChefDisplayMarkers`
  (params (CurrentMarker :type "Actor Object Reference"))
  (bind _markertype (message `/Game/GuideMarkerGUI/BPI_GuideMarkerHolder.GetMarkerType` CurrentMarker))
  (if (`KismetStringLibrary.EqualEqual_StrStr` (`self.LastAction`) "GotIngredient ")
    (if (`KismetStringLibrary.EqualEqual_StrStr` _markertype "Ingredient")
      (message `/Game/GuideMarkerGUI/BPI_GuideMarkerHolder.HideMarker` CurrentMarker)
      (else
        (bind _returnvalue (`self.GetLastOrderBrush`))
        (if (and (`KismetStringLibrary.EqualEqual_StrStr` _markertype "Blacksmith") (== _returnvalue "/Game/Orders/T_BlacksmithFinal.T_BlacksmithFinal"))
          (message `/Game/GuideMarkerGUI/BPI_GuideMarkerHolder.DisplayMarker` CurrentMarker)
          (else
            (bind _returnvalue_2 (`self.GetLastOrderBrush`))
            (if (and (`KismetStringLibrary.EqualEqual_StrStr` _markertype "Fishing") (== _returnvalue_2 "/Game/Orders/T_FishingFinal.T_FishingFinal"))
              (message `/Game/GuideMarkerGUI/BPI_GuideMarkerHolder.DisplayMarker` CurrentMarker)
              (else
                (bind _returnvalue_3 (`self.GetLastOrderBrush`))
                (if (and (`KismetStringLibrary.EqualEqual_StrStr` _markertype "Mixing") (== _returnvalue_3 "/Game/Orders/T_MixingFinal.T_MixingFinal"))
                  (message `/Game/GuideMarkerGUI/BPI_GuideMarkerHolder.DisplayMarker` CurrentMarker)
                  (elif (not (`KismetStringLibrary.EqualEqual_StrStr` _markertype "ServeDish"))
                    (message `/Game/GuideMarkerGUI/BPI_GuideMarkerHolder.HideMarker` CurrentMarker)))))))))
    (elif (`KismetStringLibrary.EqualEqual_StrStr` (`self.LastAction`) "StartedMinigame ")
      (if (`KismetStringLibrary.EqualEqual_StrStr` _markertype "Blacksmith")
        (message `/Game/GuideMarkerGUI/BPI_GuideMarkerHolder.HideMarker` CurrentMarker :!label _label)
        (elif (`KismetStringLibrary.EqualEqual_StrStr` _markertype "Fishing")
          (goto _label)
          (elif (`KismetStringLibrary.EqualEqual_StrStr` _markertype "Mixing")
            (goto _label))))
      (elif (`KismetStringLibrary.EqualEqual_StrStr` (`self.LastAction`) "CompletedMeal")
        (if (`KismetStringLibrary.EqualEqual_StrStr` _markertype "ServeDish")
          (message `/Game/GuideMarkerGUI/BPI_GuideMarkerHolder.DisplayMarker` CurrentMarker))
        (elif (`KismetStringLibrary.EqualEqual_StrStr` (`self.LastAction`) "ServedMeal")
          (if (`KismetStringLibrary.EqualEqual_StrStr` _markertype "ServeDish")
            (message `/Game/GuideMarkerGUI/BPI_GuideMarkerHolder.HideMarker` CurrentMarker)
            (elif (`KismetStringLibrary.EqualEqual_StrStr` _markertype "Ingredient")
              (message `/Game/GuideMarkerGUI/BPI_GuideMarkerHolder.DisplayMarker` CurrentMarker))))))))

(fn `GetLastOrderBrush`
  (returns (ReturnValue :type "Texture2D Object Reference"))
  (return (`WidgetBlueprintLibrary.GetBrushResourceAsTexture2D` (`Image.Brush` (`/Game/Orders/UI_OrderGui.Image` (`/Game/Orders/BP_Order.ThisOrderGui` (`/Game/Orders/BP_OrderManager.LowestTimedOrder` (`self.OrderManager`))))))))

(fn `MarkerDisplayCheck`
  (params (CurrentMarker :type "Actor Object Reference") (WhichActor :type "/Game/ThirdPerson/Blueprints/BP_BaseCharacter Object Reference") (ExtraActor :type "/Game/ThirdPerson/Blueprints/BP_BaseCharacter Object Reference"))
  (message `/Game/GuideMarkerGUI/BPI_GuideMarkerHolder.SetMarkerOwner` CurrentMarker WhichActor)
  (if (not (== WhichActor "/Game/ThirdPerson/Blueprints/BP_RatCharacter.BP_RatCharacter"))
    (`self.ChefDisplayMarkers` CurrentMarker)))

(fn `UserConstructionScript`)
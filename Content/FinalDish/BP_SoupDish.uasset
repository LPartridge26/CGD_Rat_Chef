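; BP_SoupDish is a soup dish Blueprint in the FinalDish folder that answers prompt and state queries for the Chef and Rat characters.
; Both prompt-type getters return its ObjectType, while the pipe and wire state getters always return false for either character.
; Its construction script only calls the parent's, and the file adds no other logic.
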(fn `Chef_GetPipesState`
  (returns (PipeState :type Boolean))
  (return false))

(fn `Chef_GetPromptType`
  (returns (PromptType :type String))
  (return (`self.ObjectType`)))

(fn `Chef_GetWireState`
  (returns (WireState :type Boolean))
  (return false))

(fn `Rat_GetPipesState`
  (returns (PipeState :type Boolean))
  (return false))

(fn `Rat_GetPromptType`
  (returns (PromptType :type String))
  (return (`self.ObjectType`)))

(fn `Rat_GetWiresState`
  (returns (WireState :type Boolean))
  (return false))

(fn `UserConstructionScript`
  (`parent.UserConstructionScript`))
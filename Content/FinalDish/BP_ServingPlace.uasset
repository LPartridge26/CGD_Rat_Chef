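; Serving spot where the player delivers a finished dish to fulfil an order.
; On overlap, it checks that the character holds an item tagged FinalDish, then broadcasts ServingFood with a DeletingOrder flag blocking repeat triggers.
; OrderFound clears the served dish through the character and adds fixed score via BP_ScoreManager, while OrderNotFound and OrderDeleted release the flag.
; Input prompt and guide marker start hidden and toggle through events.
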(event `self.ReceiveBeginPlay`
  ;[1 1 1] Get refrences
  (bind _returnvalue (`GameplayStatics.GetActorOfClass` "/Game/ThirdPerson/Blueprints/BP_ThirdPersonCharacter.BP_ThirdPersonCharacter_C"))
  (set `self.CharacterRefrence` _returnvalue)
  (bind _returnvalue_2 (`GameplayStatics.GetActorOfClass` "/Game/Managers/BP_ScoreManager.BP_ScoreManager_C"))
  (set `self.ScoreRefrence` _returnvalue_2)
  (`SceneComponent.SetVisibility` (`self.InputPrompt`) false false)
  (`SceneComponent.SetVisibility` (`self.GuideMarker`) false false))

(event `self.ReceiveActorBeginOverlap`
  (params (OtherActor :type "Actor Object Reference"))
  (if (not (`self.DeletingOrder`))
    (set `self.DeletingOrder` true)
    ;[1 1 1] If all the checks are met then the fianl order is served
    (bind _asbp_third_person_character (cast `/Game/ThirdPerson/Blueprints/BP_ThirdPersonCharacter` OtherActor)
      (:`then`
        (bind _output_get (set `self.CharacterRefrence` _asbp_third_person_character))
        (bind _itemreference (`/Game/ThirdPerson/Blueprints/BP_ThirdPersonCharacter.ItemReference` _output_get))
        (if (`KismetSystemLibrary.IsValid` _itemreference)
          (if (and (`self.ActorHasTag` _itemreference "FinalDish") (`/Game/ThirdPerson/Blueprints/BP_ThirdPersonCharacter.HasItem` _output_get))
            (`self.ServingFood` _itemreference)
            (else
              (set `self.DeletingOrder` false)))
          (else
            (set `self.DeletingOrder` false))))
      (:`CastFailed`
        (set `self.DeletingOrder` false)))))

(event `OrderFound`
  ;[1 1 1] Adding score
  (`/Game/ThirdPerson/Blueprints/BP_ThirdPersonCharacter.ServedFinalDish` (stale `self.ReceiveActorBeginOverlap` _output_get))
  (bind _asbp_score_manager (cast `/Game/Managers/BP_ScoreManager` (`self.ScoreRefrence`)))
  (`/Game/Managers/BP_ScoreManager.AddScoreSimple` _asbp_score_manager 25))

(event `OrderNotFound`
  (set `self.DeletingOrder` false))

(event `OrderDeleted`
  (set `self.DeletingOrder` false))

(event `self.Box.OnComponentBeginOverlap`
  (params (OverlappedComponent :type "PrimitiveComponent Object Reference") (OtherActor :type "Actor Object Reference") (OtherComp :type "PrimitiveComponent Object Reference") (OtherBodyIndex :type Integer) (bFromSweep :type Boolean) (SweepResult :type "HitResult Structure (by ref)")))

(event `/Game/InputPromptUI/BPI_Chef_InputPrompt_Holder.HidePrompt`
  (`SceneComponent.SetVisibility` (`self.InputPrompt`) false false))

(event `/Game/InputPromptUI/BPI_Chef_InputPrompt_Holder.DisplayPrompt`
  (`SceneComponent.SetVisibility` (`self.InputPrompt`) true false))

(event `/Game/GuideMarkerGUI/BPI_GuideMarkerHolder.HideMarker`
  (`SceneComponent.SetVisibility` (`self.GuideMarker`) false false))

(event `/Game/GuideMarkerGUI/BPI_GuideMarkerHolder.DisplayMarker`
  (`SceneComponent.SetVisibility` (`self.GuideMarker`) true false))

(fn `GetMarkerType`
  (returns (MarkerType :type String))
  (return (`self.MarkerType`)))

(fn `InputPrompt_GetActorOwner`
  (returns (ActorName :type String))
  (return (`self.Actor Owner`)))

(fn `Marker_GetActorOwner`
  (returns (ActorName :type String))
  (return (`self.Actor Owner`)))

(fn `UserConstructionScript`)
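; BP_StopSign is a sign actor that moves vertically, rising or lowering by a fixed height when another object calls LerpSignUp or LerpSignDown.
; Each event stores an offset target transform, then plays its own timeline to lerp the actor toward it.
; The blend starts from the actor's current transform every update rather than a saved start, so motion compounds toward the target.
; Each timeline rewinds on finish for reuse.
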(event `LerpSignUp`
  (bind (_returnvalue_location _returnvalue_rotation _returnvalue_scale) (`KismetMathLibrary.BreakTransform` (`self.GetTransform` self)))
  ;[1 1 1] Lerp sign up
  (set `self.LerpTransform` (`KismetMathLibrary.MakeTransform` (+ _returnvalue_location (0.0 0.0 250.0)) _returnvalue_rotation _returnvalue_scale))
  (bind (_direction _alpha) (`Timeline|Lerp Sign Up`)
    (:`Update`
      (`self.K2_SetActorTransform` self (`KismetMathLibrary.TLerp` (`self.GetTransform` self) (`self.LerpTransform`) _alpha) false false))
    (:`Finished`
      (`TimelineComponent.SetNewTime` (`self.Lerp Sign Up`) 0.0))))

(event `LerpSignDown`
  (bind (_returnvalue_location _returnvalue_rotation _returnvalue_scale) (`KismetMathLibrary.BreakTransform` (`self.GetTransform` self)))
  ;[1 1 1] Lerp sign down
  (set `self.LerpTransform` (`KismetMathLibrary.MakeTransform` (- _returnvalue_location (0.0 0.0 250.0)) _returnvalue_rotation _returnvalue_scale))
  (bind (_direction _alpha) (`Timeline|Lerp Sign Down`)
    (:`Update`
      (`self.K2_SetActorTransform` self (`KismetMathLibrary.TLerp` (`self.GetTransform` self) (`self.LerpTransform`) _alpha) false false))
    (:`Finished`
      (`TimelineComponent.SetNewTime` (`self.Lerp Sign Down`) 0.0))))

(fn `UserConstructionScript`)
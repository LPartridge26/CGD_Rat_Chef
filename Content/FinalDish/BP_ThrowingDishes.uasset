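; BP_ThrowingDishes lets a chef throw a finished dish they are holding.
; Its ThrowFood event checks that the given chef holds a valid item tagged FinalDish, stores it and makes the chef drop it.
; It then applies an impulse to the dish's ItemModel along the chef's forward vector scaled by ThrowForce, plus a fixed upward boost.
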(event `self.ReceiveBeginPlay`)

(event `self.ReceiveTick`
  (params (DeltaSeconds :type "Float (single-precision)")))

(event `ThrowFood`
  (params (Chef :type "/Game/ThirdPerson/Blueprints/BP_ThirdPersonCharacter Object Reference"))
  (bind _itemreference (`/Game/ThirdPerson/Blueprints/BP_ThirdPersonCharacter.ItemReference` Chef))
  (if (and (`/Game/ThirdPerson/Blueprints/BP_ThirdPersonCharacter.HasItem` Chef) (`KismetSystemLibrary.IsValid` _itemreference))
    (if (`self.ActorHasTag` _itemreference "FinalDish")
      (set `self.FoodToThrow` _itemreference)
      (`/Game/ThirdPerson/Blueprints/BP_ThirdPersonCharacter.Drop Item` Chef)
      (`PrimitiveComponent.AddImpulse` (`/Game/PickUpable/Blueprints/BP_PickUp_Item.ItemModel` (`self.FoodToThrow`)) (+ (* (`self.GetActorForwardVector` Chef) (`self.ThrowForce`)) (0.0 0.0 50000.0)) "None" false))))

(fn `UserConstructionScript`)
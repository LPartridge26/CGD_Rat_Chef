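; Minigame station Blueprint that tracks whether the Chef or the Rat owns it and shows its state through the MinigameArea material.
; Interact turns the area yellow and Exit turns it red.
; Chef completion turns it green and claims ownership; Rat completion turns it red, claims ownership and spawns RatFood at FoodSpawn.
; Check functions let the Chef play unless it owns the station, and the Rat only when the Chef does.
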(event `/Game/MiniGameInteractiveControls/BPI_MiniGameObject.Interact`
  (`PrimitiveComponent.SetMaterial` (`self.MinigameArea`) 0 "/Game/MiniGameInteractiveControls/M_Yellow.M_Yellow"))

(event `/Game/MiniGameInteractiveControls/BPI_MiniGameObject.Exit`
  (`PrimitiveComponent.SetMaterial` (`self.MinigameArea`) 0 "/Game/MiniGameInteractiveControls/M_Red.M_Red"))

(event `/Game/MiniGameInteractiveControls/BPI_MiniGameObject.Chef_Complete`
  (`PrimitiveComponent.SetMaterial` (`self.MinigameArea`) 0 "/Game/MiniGameInteractiveControls/M_Green.M_Green")
  (set `self.MinigameOwner` "Chef"))

(event `/Game/MiniGameInteractiveControls/BPI_MiniGameObject.Rat_Complete`
  (`PrimitiveComponent.SetMaterial` (`self.MinigameArea`) 0 "/Game/MiniGameInteractiveControls/M_Red.M_Red")
  (set `self.MinigameOwner` "Rat")
  (`|SpawnActorFromClass` "/Game/ThirdPerson/Blueprints/RatFood.RatFood_C" (`KismetMathLibrary.Conv_VectorToTransform` (`SceneComponent.K2_GetComponentLocation` (`self.FoodSpawn`))) "Undefined" "MultiplyWithRoot" null null))

(fn `Chef_MiniGameCheck`
  (returns (CanStartGame :type Boolean))
  (if (`KismetStringLibrary.EqualEqual_StrStr` (`self.MinigameOwner`) "Chef")
    (set `self.GamePossible` false)
    (else
      (set `self.GamePossible` true)))
  (return (`self.GamePossible`)))

(fn `Rat_MiniGameCheck`
  (returns (CanStartGame :type Boolean))
  (if (`KismetStringLibrary.EqualEqual_StrStr` (`self.MinigameOwner`) "Chef")
    (set `self.GamePossible` true)
    (else
      (set `self.GamePossible` false)))
  (return (`self.GamePossible`)))

(fn `UserConstructionScript`)
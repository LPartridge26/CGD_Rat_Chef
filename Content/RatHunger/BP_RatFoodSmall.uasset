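; BP_RatFoodSmall is a small food pickup in the rat hunger system, built as a child of a parent food Blueprint.
; On BeginPlay it marks itself visible and takes its food quality from FoodQualityL, while overlap handling is left to the parent.
; Its FoodEaten override calls the parent, tells the HungerComponent to eat it straight away at that quality, then hides the food.
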(event `self.ReceiveBeginPlay`
  (set `self.Is Visible` true)
  (set `self.Food Quality` (`self.Food Quality L`)))

(event `self.ReceiveActorBeginOverlap`
  (params (OtherActor :type "Actor Object Reference"))
  (`parent.ReceiveActorBeginOverlap` OtherActor))

(fn `Food Eaten`
  (params (`Hunger Component` :type "/Game/RatHunger/BP_HungerComponent Object Reference") (`Has Food` :type Boolean))
  (`parent.Food Eaten` `Hunger Component` false)
  (`/Game/RatHunger/BP_HungerComponent.Food Eaten` `Hunger Component` true (`self.Food Quality`))
  (`self.Toggle Visible` false))

(fn `UserConstructionScript`
  (`parent.UserConstructionScript`))
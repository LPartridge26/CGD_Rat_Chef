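; Hunger component for BP_RatCharacter that manages hunger, a single carried food, sprinting and their per-player UI.
; Round restart builds the UI and starts a self-recalling delayed loop that drains hunger and sets walk speed, slowing below zero.
; Eating stuns the rat before restoring hunger, while sprinting spends hunger for timed speed, both with Niagara effects.
; Tick updates the hunger bar and rebuilds widgets when the game mode's Toggle changes.
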(event `Sprint`
  ;[1 1 1] Handles Sprinting
  (set `self.Hunger Value` (- (`self.Hunger Value`) (`self.Food Value For Sprint`)))
  (set `self.Is Sprinting` true)
  (set `CharacterMovementComponent.MaxWalkSpeed` (`self.Sprint Speed`) (`Character.CharacterMovement` (`self.Owner `)))
  (bind _returnvalue (`NiagaraFunctionLibrary.SpawnSystemAttached` "/Game/ThirdPerson/Effects/FX_SprintParticle.FX_SprintParticle" (`Character.CapsuleComponent` (`self.Owner `)) "None" (0.0 0.0 0.0) (struct) "KeepRelativeOffset"))
  (`KismetSystemLibrary.Delay` (`self.Sprint Time`))
  (`self.K2_DestroyComponent` _returnvalue)
  (set `CharacterMovementComponent.MaxWalkSpeed` (`self.Normal Walk Speed`) (`Character.CharacterMovement` (`self.Owner `)))
  (set `self.Is Sprinting` false))

(event `Eating Timer`
  ;[1 1 1] Handles Eating
  (bind _returnvalue (`NiagaraFunctionLibrary.SpawnSystemAttached` "/Game/ThirdPerson/Effects/FX_EatingCheese.FX_EatingCheese" (`Character.CapsuleComponent` (`self.Owner `)) "None" (0.0 0.0 0.0) (struct) "KeepRelativeOffset"))
  (set `/Game/ThirdPerson/Blueprints/BP_RatCharacter.Stunned` true (`self.Owner `))
  (set `/Game/ThirdPerson/Blueprints/BP_RatCharacter.Stunned Timer` (`self.Max eat time`) (`self.Owner `))
  (`KismetSystemLibrary.Delay` (`self.Max eat time`))
  (`self.Food Eaten` false (`self.Food Quality`))
  (`self.K2_DestroyComponent` _returnvalue))

(event `Hunger Decrement`
  (bind _charactermovement (`Character.CharacterMovement` (`self.Owner `)))
  ;[1 1 1] Decrements hunger and sets walk speed accordingly
  (`KismetSystemLibrary.Delay` (`self.Interval Time`))
  (if (>= (`self.Hunger Value`) 0)
    (set `CharacterMovementComponent.MaxWalkSpeed` (`self.Normal Walk Speed`) _charactermovement)
    (`/Engine/EditorBlueprintResources/StandardMacros.DecrementInt` (`self.Hunger Value`)
      (:`  `
        (`self.Hunger Decrement `)))
    (else
      (set `CharacterMovementComponent.MaxWalkSpeed` (`self.Low Hunger Speed`) _charactermovement)
      (`self.Hunger Decrement `))))

(event `self.ReceiveBeginPlay`
  (bind _asbp_rat_character (cast `/Game/ThirdPerson/Blueprints/BP_RatCharacter` (`self.GetOwner`)))
  (set `self.Owner ` _asbp_rat_character)
  (bind _asbp_third_person_game_mode (cast `/Game/ThirdPerson/Blueprints/BP_ThirdPersonGameMode` (`GameplayStatics.GetGameMode`)))
  (set `self.Toggle Local` (`/Game/ThirdPerson/Blueprints/BP_ThirdPersonGameMode.Toggle` _asbp_third_person_game_mode)))

(event `self.ReceiveTick`
  (params (DeltaSeconds :type "Float (single-precision)"))
  (`KismetSystemLibrary.Delay` 0.1)
  (`self.Send percent to Hunger Bar`)
  (`self.Check UI state`))

(event `EnhancedInput|/Game/ThirdPerson/Input/Default_Actions/IA_RatEat`
  (params (ActionValue :type Boolean) (ElapsedSeconds :type "Float (double-precision)") (TriggeredSeconds :type "Float (double-precision)") (InputAction :type "InputAction Object Reference" :default "/Game/ThirdPerson/Input/Default_Actions/IA_RatEat.IA_RatEat"))
  (:`Started`
    (if (`self.Has Food`)
      (`self.Eating Timer`))))

(event `EnhancedInput|/Game/ThirdPerson/Input/Default_Actions/IA_RatSprint`
  (params (ActionValue :type Boolean) (ElapsedSeconds :type "Float (double-precision)") (TriggeredSeconds :type "Float (double-precision)") (InputAction :type "InputAction Object Reference" :default "/Game/ThirdPerson/Input/Default_Actions/IA_RatSprint.IA_RatSprint"))
  (:`Started`
    (`self.Sprint Check`)))

(fn `Check UI state`
  (bind _asbp_third_person_game_mode (cast `/Game/ThirdPerson/Blueprints/BP_ThirdPersonGameMode` (`GameplayStatics.GetGameMode`)))
  (bind _toggle (`/Game/ThirdPerson/Blueprints/BP_ThirdPersonGameMode.Toggle` _asbp_third_person_game_mode))
  (if (not (== _toggle (`self.Toggle Local`)))
    (set `self.Toggle Local` _toggle)
    (`self.Destroy UI`)
    (`self.Create UI `)))

(fn `Create UI `
  (locals (Controller :type "PlayerController Object Reference"))
  (bind _asplayer_controller (cast `PlayerController` (`Pawn.GetController` (`self.Owner `))))
  (bind _output_get (set `local.Controller` _asplayer_controller))
  (bind _returnvalue (`|CreateWidget` "/Game/RatHunger/UI_RatInventory.UI_RatInventory_C" _output_get))
  (bind _output_get_2 (set `self.Slot Widget` _returnvalue))
  (`UserWidget.AddToPlayerScreen` _output_get_2 0)
  (bind _returnvalue_2 (`|CreateWidget` "/Game/RatHunger/UI_HungerBarTile.UI_HungerBarTile_C" (`local.Controller`)))
  (bind _output_get_3 (set `self.Hunger Bar` _returnvalue_2))
  (`UserWidget.AddToPlayerScreen` _output_get_3 0))

(fn `Destroy UI`
  (bind _slot_widget (`self.Slot Widget`)
    (:`then`
      (`Widget.RemoveFromParent` _slot_widget)
      (bind _hunger_bar (`self.Hunger Bar`)
        (:`then`
          (`Widget.RemoveFromParent` _hunger_bar))
        (:`else`)))
    (:`else`)))

(fn `Food Collected`
  (params (`Food Quality` :type "Float (double-precision)"))
  (set `self.Food Quality` `Food Quality`)
  (set `self.Has Food` true)
  (`self.Food Collected UI`))

(fn `Food Collected UI`
  (`UserWidget.SetColorAndOpacity` (`self.Slot Widget`) (`self.Has Food Color`)))

(fn `Food Eaten`
  (params (`Eat Straight Away` :type Boolean) (`Food Quality` :type "Float (double-precision)"))
  (set `self.Hunger Value` (+ `Food Quality` (`self.Hunger Value`)))
  (set `self.Has Food` false)
  (`self.Food Eaten UI`))

(fn `Food Eaten UI`
  (`UserWidget.SetColorAndOpacity` (`self.Slot Widget`) (`self.No Food Color`)))

(fn `On Round Restart`
  (`self.Create UI `)
  (`self.Food Eaten UI`)
  (`self.Reset Values`)
  (`self.Hunger Decrement `))

(fn `On Round Stop`
  (`self.Destroy UI`))

(fn `Reset Values`
  (set `self.Hunger Value` (`self.Max Hunger`))
  (set `self.Interval Time` (`self.Normal interval time`)))

(fn `Send percent to Hunger Bar`
  (`self.Hunger Bar`
    (:`then`
      (`/Game/RatHunger/UI_HungerBarTile.Set Percent` (`self.Hunger Bar`) (/ (`KismetMathLibrary.Conv_IntToDouble` (`self.Hunger Value`)) 10.0)))
    (:`else`)))

(fn `Sprint Check`
  (if (`self.Is Sprinting`)
    _
    (elif (>= (`self.Hunger Value`) (`self.Food Value For Sprint`))
      (`self.Sprint`))))

(fn `UI Toggle`
  (`self.Slot Widget`
    (:`then`
      (bind _asbp_third_person_game_mode (cast `/Game/ThirdPerson/Blueprints/BP_ThirdPersonGameMode` (`GameplayStatics.GetGameMode`)))
      (if (`/Game/ThirdPerson/Blueprints/BP_ThirdPersonGameMode.Toggle` _asbp_third_person_game_mode)
        (`UserWidget.SetPositionInViewport` (`self.Slot Widget`) (300.0 1000.0) true)
        (else
          (`UserWidget.SetPositionInViewport` (`self.Slot Widget`) (3000.0 1000.0) true)))
      (bind _asbp_third_person_game_mode_2 (cast `/Game/ThirdPerson/Blueprints/BP_ThirdPersonGameMode` (`GameplayStatics.GetGameMode`)))
      (if (`/Game/ThirdPerson/Blueprints/BP_ThirdPersonGameMode.Toggle` _asbp_third_person_game_mode_2)
        (`UserWidget.SetPositionInViewport` (`self.Hunger Bar`) (0.0 0.0) true)
        (else
          (`UserWidget.SetPositionInViewport` (`self.Hunger Bar`) (1400.0 0.0) true))))
    (:`else`)))
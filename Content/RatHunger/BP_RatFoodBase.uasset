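; BP_RatFoodBase is a base food pickup for the rat character, shown as bobbing cheese.
; Tick moves the cheese up and down on a sine wave around its starting relative location.
; While visible, overlap with a rat passes its hunger component and HasFood state to FoodEaten, which is empty here.
; ToggleVisible sets both the visibility flag and whether the actor is hidden.
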(event `self.ReceiveBeginPlay`
  (set `self.CheeseRelativeLocation` (`SceneComponent.RelativeLocation` (`self.Cheese`))))

(event `self.ReceiveActorBeginOverlap`
  (params (OtherActor :type "Actor Object Reference"))
  (if (`self.Is Visible`)
    (bind _asbp_rat_character (cast `/Game/ThirdPerson/Blueprints/BP_RatCharacter` OtherActor))
    (bind _output_get (set `self.Hunger Component` (`/Game/ThirdPerson/Blueprints/BP_RatCharacter.BP_HungerComponent` _asbp_rat_character)))
    (`self.Food Eaten` _output_get (`/Game/RatHunger/BP_HungerComponent.Has Food` _output_get))))

(event `self.ReceiveTick`
  (params (DeltaSeconds :type "Float (single-precision)"))
  (bind (_cheeserelativelocation_x _cheeserelativelocation_y _cheeserelativelocation_z) (`KismetMathLibrary.BreakVector` (`self.CheeseRelativeLocation`)))
  (`SceneComponent.K2_SetRelativeLocation` (`self.Cheese`) (`KismetMathLibrary.MakeVector` _cheeserelativelocation_x _cheeserelativelocation_y (+ _cheeserelativelocation_z (* (+ (`KismetMathLibrary.DegSin` (* (`self.GetGameTimeSinceCreation`) (`self.BobbingSpeed`))) 1.5) (`self.BobbingDistance`)))) false false))

(fn `Food Eaten`
  (params (`Hunger Component` :type "/Game/RatHunger/BP_HungerComponent Object Reference") (`Has Food` :type Boolean)))

(fn `Toggle Visible`
  (params (Visible :type Boolean))
  (bind _output_get (set `self.Is Visible` Visible))
  (`self.SetActorHiddenInGame` (not _output_get)))

(fn `UserConstructionScript`)
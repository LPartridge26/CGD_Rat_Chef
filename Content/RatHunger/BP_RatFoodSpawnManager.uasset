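; Spawn manager for the RatHunger game that rotates which pre-placed BP_RatFood actors are visible.
; BeginPlay caches every food actor, and OnRoundRestart starts a self-repeating Timer event spaced by a Delay of IntervalLength.
; Each cycle hides all food, then shows MaxActive random picks by toggling visibility instead of spawning.
; Picks can repeat, so fewer than MaxActive items may appear.
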(event `Timer`
  (`self.Set food visible`)
  (`KismetSystemLibrary.Delay` (`self.Interval Length`))
  (`self.Timer`))

(event `self.ReceiveBeginPlay`
  (bind _outactors (`GameplayStatics.GetAllActorsOfClass` "/Game/RatHunger/BP_RatFood.BP_RatFood_C"))
  (set `self.Food Array` _outactors))

(fn `Clear all food`
  (for _array_element (`self.Food Array`)
    (`/Game/RatHunger/BP_RatFood.Toggle Visible` _array_element false)))

(fn `On Round Restart`
  (`self.Timer`))

(fn `Set food visible`
  (locals (`index rand` :type Integer))
  (`self.Clear all food`)
  (set `local.index rand` 0)
  (for _ (range 1 (+ (`self.Max Active`) 1))
    (bind _output_get (set `local.index rand` (`KismetMathLibrary.RandomInteger` (`KismetArrayLibrary.Array_Length` (`self.Food Array`)))))
    (bind _asbp_rat_food (cast `/Game/RatHunger/BP_RatFood` (`|GetArrayItem` (`self.Food Array`) _output_get)))
    (`/Game/RatHunger/BP_RatFood.Toggle Visible` _asbp_rat_food true))
  (`KismetSystemLibrary.PrintString` "Looped through values"))

(fn `UserConstructionScript`)
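; BP_RatFoodBig is the large food pickup in the rat hunger system, built on a parent that handles overlap.
; On BeginPlay it sets its quality to the large value and caches the first BP_RatFoodSpawnManager in the level.
; When eaten by a rat not already holding food, it reports its quality to the hunger component, hides itself and asks the manager to shuffle food.
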(event `self.ReceiveBeginPlay`
  (set `self.Food Quality` (`self.Food Quality L`))
  (bind _outactors (`GameplayStatics.GetAllActorsOfClass` "/Game/RatHunger/BP_RatFoodSpawnManager.BP_RatFoodSpawnManager_C"))
  (set `self.Spawn Manager` (`|GetArrayItem` _outactors)))

(event `self.ReceiveActorBeginOverlap`
  (params (OtherActor :type "Actor Object Reference"))
  (`parent.ReceiveActorBeginOverlap` OtherActor))

(fn `Food Eaten`
  (params (`Hunger Component` :type "/Game/RatHunger/BP_HungerComponent Object Reference") (`Has Food` :type Boolean))
  (if (not `Has Food`)
    (`/Game/RatHunger/BP_HungerComponent.Food Collected` `Hunger Component` (`self.Food Quality`))
    (`self.Toggle Visible` false)
    (`/Game/RatHunger/BP_RatFoodSpawnManager.Shuffle Food` (`self.Spawn Manager`))))

(fn `UserConstructionScript`
  (`parent.UserConstructionScript`))
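; BP_Ingredient_Spawner is an ingredient spawner actor that so far only handles highlighting, with no spawn logic.
; When a BP_ThirdPersonCharacter begins overlapping its Detectbox, an outline overlay material is applied if both the character's SightBox and RangeBox overlap it.
; The check runs only on begin overlap, and any end overlap on Detectbox clears the overlay, regardless of which actor or component left.
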(event `self.Detectbox.OnComponentBeginOverlap`
  (params (OverlappedComponent :type "PrimitiveComponent Object Reference") (OtherActor :type "Actor Object Reference") (OtherComp :type "PrimitiveComponent Object Reference") (OtherBodyIndex :type Integer) (bFromSweep :type Boolean) (SweepResult :type "HitResult Structure (by ref)"))
  (bind _asbp_third_person_character (cast `/Game/ThirdPerson/Blueprints/BP_ThirdPersonCharacter` OtherActor))
  (if (and (`PrimitiveComponent.IsOverlappingComponent` (`self.Detectbox`) (`/Game/ThirdPerson/Blueprints/BP_ThirdPersonCharacter.Sight Box` _asbp_third_person_character)) (`PrimitiveComponent.IsOverlappingComponent` (`self.Detectbox`) (`/Game/ThirdPerson/Blueprints/BP_ThirdPersonCharacter.Range Box` _asbp_third_person_character)))
    (`MeshComponent.SetOverlayMaterial` (`self.Detectbox`) "/Game/Material/M_Outline.M_Outline")))

(event `self.Detectbox.OnComponentEndOverlap`
  (params (OverlappedComponent :type "PrimitiveComponent Object Reference") (OtherActor :type "Actor Object Reference") (OtherComp :type "PrimitiveComponent Object Reference") (OtherBodyIndex :type Integer))
  (`MeshComponent.SetOverlayMaterial` (`self.Detectbox`) null))

(fn `UserConstructionScript`)
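; Manager that shows or hides input prompts based on proximity to the Chef and Rat characters.
; SetInputPromptValues caches both characters from RoundManager and gathers every actor implementing BPI_InputPromptUI.
; InputPromptCheck reads each prompt's owner tag and passes the matching character to InputDisplayCheck, which toggles display by distance through interface messages.
; Prompts tagged Both effectively track only the Chef, since the extra Rat argument is unused.
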(event `Set InputPrompt Values`
  (bind _roundmanager (`self.RoundManager`))
  ;[0 0.1291 1 1 35] SetManagerValues
  (set `self.ChefActor` (`/Game/Managers/BP_RoundManager.Chef` _roundmanager))
  (set `self.RatActor` (`/Game/Managers/BP_RoundManager.Rat` _roundmanager))
  (bind _outactors (`GameplayStatics.GetAllActorsWithInterface` "/Game/InputPromptUI/BPI_InputPromptUI.BPI_InputPromptUI_C"))
  (bind _output_get (set `self.InputPromots` _outactors))
  (for _ _output_get
    _))

(event `InputPromptCheck`
  ;[0.2292 0.358 1 1 35] InputPromptCheck
  (for _array_element (`self.InputPromots`)
    (bind _actorname (message `/Game/InputPromptUI/BPI_InputPromptUI.GetActorOwner` _array_element))
    (if (`KismetStringLibrary.EqualEqual_StrStr` _actorname "Chef")
      (`self.InputDisplayCheck` _array_element (`self.ChefActor`))
      (elif (`KismetStringLibrary.EqualEqual_StrStr` _actorname "Rat")
        (`self.InputDisplayCheck` _array_element (`self.RatActor`))
        (elif (`KismetStringLibrary.EqualEqual_StrStr` _actorname "Both")
          (`self.InputDisplayCheck` _array_element (`self.ChefActor`) (`self.RatActor`)))))))

(fn `InputDisplayCheck`
  (params (CurrentInput :type "Actor Object Reference") (WhichActor :type "/Game/ThirdPerson/Blueprints/BP_BaseCharacter Object Reference") (ExtraActor :type "/Game/ThirdPerson/Blueprints/BP_BaseCharacter Object Reference"))
  (if (< (`KismetMathLibrary.VSize` (- (`self.K2_GetActorLocation` CurrentInput) (`self.K2_GetActorLocation` WhichActor))) 205.0)
    (message `/Game/InputPromptUI/BPI_InputPromptUI.DisplayPrompt` CurrentInput)
    (else
      (message `/Game/InputPromptUI/BPI_InputPromptUI.HidePrompt` CurrentInput))))

(fn `UserConstructionScript`)
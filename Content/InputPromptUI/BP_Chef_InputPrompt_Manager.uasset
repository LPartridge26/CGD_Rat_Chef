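; Manager that shows or hides a chef's on-screen input prompt based on proximity to prompt holders and the chef's last action.
; Setup creates a hidden per-player widget and caches all BPI_Chef_InputPrompt_Holder actors, which each display check tests for distance.
; Chef events record the last action by name, but only the no-ingredient state near Ingredient holders drives visibility.
; A swap event recreates the widget for the chef's current viewing controller.
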(event `/Game/PlayerEventsBPI/BPI_ChefEvents.SetManagerValues`
  (params (ChefActor :type "/Game/ThirdPerson/Blueprints/BP_ThirdPersonCharacter Object Reference"))
  ;[0 0.1291 1 1 35] SetManagerValues
  (bind _output_get (set `self.ChefActor` ChefActor))
  (bind _returnvalue (`|CreateWidget` "/Game/InputPromptUI/UI_Chef_InputPrompts.UI_Chef_InputPrompts_C" (`Pawn.GetLocalViewingPlayerController` _output_get)))
  (bind _output_get_2 (set `self.InputPrompt` _returnvalue))
  (`UserWidget.AddToPlayerScreen` _output_get_2 0)
  (`Widget.SetVisibility` _output_get_2 "Hidden")
  (bind _outactors (`GameplayStatics.GetAllActorsWithInterface` "/Game/InputPromptUI/BPI_Chef_InputPrompt_Holder.BPI_Chef_InputPrompt_Holder_C"))
  (set `self.ChefInputPromots` _outactors))

(event `/Game/PlayerEventsBPI/BPI_ChefEvents.ManagerDisplayCheck`
  ;[0 0.1294 1 1 35] InputPromptCheck
  (for _array_element (`self.ChefInputPromots`)
    (`self.InputDisplayCheck` _array_element)))

(event `/Game/PlayerEventsBPI/BPI_ChefEvents.SwapChefUI`
  ;[0 0.1294 1 1 35] SwapScreenUI
  (`Widget.RemoveFromParent` (`self.InputPrompt`))
  (bind _returnvalue (`|CreateWidget` "/Game/InputPromptUI/UI_Chef_InputPrompts.UI_Chef_InputPrompts_C" (`Pawn.GetLocalViewingPlayerController` (`self.ChefActor`))))
  (bind _output_get (set `self.InputPrompt` _returnvalue))
  (`UserWidget.AddToPlayerScreen` _output_get 0))

(event `/Game/PlayerEventsBPI/BPI_ChefEvents.NoIngredient`
  ;[0 0.1294 1 1 35] ChefEvents
  (set `self.LastAction` "NoIngredient"))

(event `/Game/PlayerEventsBPI/BPI_ChefEvents.GotIngredient`
  ;[0 0.1294 1 1 35] ChefEvents
  (set `self.LastAction` "GotIngredient"))

(event `/Game/PlayerEventsBPI/BPI_ChefEvents.StartedMinigame`
  ;[0 0.1294 1 1 35] ChefEvents
  (set `self.LastAction` "StartedMinigame"))

(event `/Game/PlayerEventsBPI/BPI_ChefEvents.CompletedMinigame`
  ;[0 0.1294 1 1 35] ChefEvents
  (set `self.LastAction` "CompletedMinigame"))

(event `/Game/PlayerEventsBPI/BPI_ChefEvents.ExitedMinigame`
  ;[0 0.1294 1 1 35] ChefEvents
  (set `self.LastAction` "ExitedMinigame"))

(event `/Game/PlayerEventsBPI/BPI_ChefEvents.ServedMeal`
  ;[0 0.1294 1 1 35] ChefEvents
  (set `self.LastAction` "ServedMeal"))

(fn `InputDisplayCheck`
  (params (CurrentInput :type "Actor Object Reference"))
  (bind _prompttype (message `/Game/InputPromptUI/BPI_Chef_InputPrompt_Holder.GetPromptType` CurrentInput))
  (if (< (`KismetMathLibrary.VSize` (- (`self.K2_GetActorLocation` CurrentInput) (`self.K2_GetActorLocation` (`self.ChefActor`)))) 205.0)
    (if (`KismetStringLibrary.EqualEqual_StrStr` (`self.LastAction`) "NoIngredient")
      (if (`KismetStringLibrary.EqualEqual_StrStr` _prompttype "Ingredient")
        (`Widget.SetVisibility` (`self.InputPrompt`) "Visible")))
    (elif (`KismetStringLibrary.EqualEqual_StrStr` (`self.LastAction`) "NoIngredient")
      (if (`KismetStringLibrary.EqualEqual_StrStr` _prompttype "Ingredient")
        (`Widget.SetVisibility` (`self.InputPrompt`) "Hidden")))))

(fn `UserConstructionScript`)
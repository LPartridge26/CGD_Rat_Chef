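; Manager that shows and hides the rat player's on-screen input prompts near Wires and Pipes minigame objects.
; Creates the prompt widget for the rat's local player and gathers all prompt-holder interface actors once at setup.
; Each display check shows the interact prompt within range of objects whose state is false, tracking the active prompt so others don't hide it.
; Minigame events hide or restore prompts; SwapRatUI rebuilds the widget hidden.
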(event `/Game/PlayerEventsBPI/BPI_RatEvents.Rat_SetManagerValues`
  (params (RatActor :type "/Game/ThirdPerson/Blueprints/BP_RatCharacter Object Reference"))
  ;[0 0.1291 1 1 35] SetManagerValues
  (bind _output_get (set `self.Rat Actor` RatActor))
  (bind _returnvalue (`|CreateWidget` "/Game/InputPromptUI/UI_Rat_InputPrompts.UI_Rat_InputPrompts_C" (`Pawn.GetLocalViewingPlayerController` _output_get)))
  (bind _output_get_2 (set `self.InputPrompt` _returnvalue))
  (`UserWidget.AddToPlayerScreen` _output_get_2 0)
  (`Widget.SetVisibility` (`/Game/InputPromptUI/UI_Rat_InputPrompts.InteractPrompt` _output_get_2) "Hidden")
  (`Widget.SetVisibility` (`/Game/InputPromptUI/UI_Rat_InputPrompts.ExtraPrompts` (`self.InputPrompt`)) "Visible")
  (bind _outactors (`GameplayStatics.GetAllActorsWithInterface` "/Game/InputPromptUI/BPI_Rat_InputPrompt_Holder.BPI_Rat_InputPrompt_Holder_C"))
  (set `self.RatInputPromots` _outactors))

(event `/Game/PlayerEventsBPI/BPI_RatEvents.Rat_ManagerDisplayCheck`
  ;[0 0.1294 1 1 35] InputPromptCheck
  (set `self.ObjectCounter` 0)
  (for _array_element (`self.RatInputPromots`)
    (`self.InputDisplayCheck` _array_element)))

(event `/Game/PlayerEventsBPI/BPI_RatEvents.SwapRatUI`
  ;[0 0.1294 1 1 35] SwapScreenUI
  (`Widget.RemoveFromParent` (`self.InputPrompt`))
  (bind _returnvalue (`|CreateWidget` "/Game/InputPromptUI/UI_Rat_InputPrompts.UI_Rat_InputPrompts_C" (`Pawn.GetLocalViewingPlayerController` (`self.Rat Actor`))))
  (bind _output_get (set `self.InputPrompt` _returnvalue))
  (`UserWidget.AddToPlayerScreen` _output_get 0)
  (`Widget.SetVisibility` (`/Game/InputPromptUI/UI_Rat_InputPrompts.InteractPrompt` _output_get) "Hidden")
  (`Widget.SetVisibility` (`/Game/InputPromptUI/UI_Rat_InputPrompts.ExtraPrompts` (`self.InputPrompt`)) "Hidden"))

(event `/Game/PlayerEventsBPI/BPI_RatEvents.Rat_StartedMinigame`
  ;[0 0.1294 1 1 35] RatEvents
  (`Widget.SetVisibility` (`/Game/InputPromptUI/UI_Rat_InputPrompts.InteractPrompt` (`self.InputPrompt`)) "Hidden")
  (`Widget.SetVisibility` (`/Game/InputPromptUI/UI_Rat_InputPrompts.ExtraPrompts` (`self.InputPrompt`)) "Hidden")
  (set `self.LastAction` "StartedMinigame"))

(event `/Game/PlayerEventsBPI/BPI_RatEvents.Rat_EndedMinigame`
  ;[0 0.1294 1 1 35] RatEvents
  (`Widget.SetVisibility` (`/Game/InputPromptUI/UI_Rat_InputPrompts.InteractPrompt` (`self.InputPrompt`)) "Hidden")
  (`Widget.SetVisibility` (`/Game/InputPromptUI/UI_Rat_InputPrompts.ExtraPrompts` (`self.InputPrompt`)) "Visible")
  (set `self.LastAction` "EndedMinigame"))

(fn `GetPlayerDistance`
  (params (`Current Input` :type "Actor Object Reference") (Distance :type "Float (double-precision)"))
  (returns (ReturnValue :type Boolean))
  (return (< (`KismetMathLibrary.VSize` (- (`self.K2_GetActorLocation` `Current Input`) (`self.K2_GetActorLocation` (`self.Rat Actor`)))) Distance)))

(fn `InputDisplayCheck`
  (params (CurrentInput :type "Actor Object Reference"))
  (bind _interactprompt (`/Game/InputPromptUI/UI_Rat_InputPrompts.InteractPrompt` (`self.InputPrompt`)))
  (bind _output_get (set `self.CurrentInputPrompt` CurrentInput))
  (bind _prompttype (message `/Game/InputPromptUI/BPI_Rat_InputPrompt_Holder.Rat_GetPromptType` _output_get))
  (set `self.CurrentPromptType` _prompttype)
  (if (`KismetStringLibrary.EqualEqual_StrStr` (`self.CurrentPromptType`) "Wires")
    (set `self.ObjectCounter` (+ (`self.ObjectCounter`) 1))
    (bind _wirestate (message `/Game/InputPromptUI/BPI_Rat_InputPrompt_Holder.Rat_GetWiresState` (`self.CurrentInputPrompt`)))
    (if _wirestate
      _
      (elif (`KismetStringLibrary.EqualEqual_StrStr` (`self.LastAction`) "StartedMinigame")
        (`Widget.SetVisibility` (`/Game/InputPromptUI/UI_Rat_InputPrompts.InteractPrompt` (`self.InputPrompt`)) "Hidden")
        (`Widget.SetVisibility` (`/Game/InputPromptUI/UI_Rat_InputPrompts.ExtraPrompts` (`self.InputPrompt`)) "Hidden")
        (else
          (bind _returnvalue (`self.GetPlayerDistance` (`self.CurrentInputPrompt`) (`self.CommonDistance`)))
          (if _returnvalue
            (`Widget.SetVisibility` (`/Game/InputPromptUI/UI_Rat_InputPrompts.InteractPrompt` (`self.InputPrompt`)) "Visible")
            (set `self.FoundPrompt` true)
            (set `self.ActivePrompt` (`KismetStringLibrary.Concat_StrStr` "Wires" (`KismetStringLibrary.Conv_IntToString` (`self.ObjectCounter`))))
            (elif (`self.FoundPrompt`)
              (if (`KismetStringLibrary.EqualEqual_StrStr` (`self.ActivePrompt`) (`KismetStringLibrary.Concat_StrStr` "Wires" (`KismetStringLibrary.Conv_IntToString` (`self.ObjectCounter`))))
                (`Widget.SetVisibility` (`/Game/InputPromptUI/UI_Rat_InputPrompts.InteractPrompt` (`self.InputPrompt`)) "Hidden"))
              (else
                (`Widget.SetVisibility` (`/Game/InputPromptUI/UI_Rat_InputPrompts.InteractPrompt` (`self.InputPrompt`)) "Hidden")
                (set `self.FoundPrompt` false)))))))
    (elif (`KismetStringLibrary.EqualEqual_StrStr` (`self.CurrentPromptType`) "Pipes")
      (bind _pipestate (message `/Game/InputPromptUI/BPI_Rat_InputPrompt_Holder.Rat_GetPipesState` (`self.CurrentInputPrompt`)))
      (if _pipestate
        _
        (elif (`KismetStringLibrary.EqualEqual_StrStr` (`self.LastAction`) "StartedMinigame")
          (`Widget.SetVisibility` (`/Game/InputPromptUI/UI_Rat_InputPrompts.InteractPrompt` (`self.InputPrompt`)) "Hidden")
          (`Widget.SetVisibility` (`/Game/InputPromptUI/UI_Rat_InputPrompts.ExtraPrompts` (`self.InputPrompt`)) "Hidden")
          (else
            (bind _returnvalue_2 (`self.GetPlayerDistance` (`self.CurrentInputPrompt`) (- (`self.CommonDistance`) 30.0)))
            (if _returnvalue_2
              (`Widget.SetVisibility` (`/Game/InputPromptUI/UI_Rat_InputPrompts.InteractPrompt` (`self.InputPrompt`)) "Visible")
              (set `self.FoundPrompt` true)
              (set `self.ActivePrompt` "Pipes")
              (elif (`self.FoundPrompt`)
                (if (`KismetStringLibrary.EqualEqual_StrStr` (`self.ActivePrompt`) "Pipes")
                  (`Widget.SetVisibility` _interactprompt "Hidden"))
                (else
                  (`Widget.SetVisibility` _interactprompt "Hidden")
                  (set `self.FoundPrompt` false))))))))))

(fn `UserConstructionScript`)
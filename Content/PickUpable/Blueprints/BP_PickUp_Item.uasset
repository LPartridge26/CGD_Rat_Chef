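; BP_PickUp_Item is a pickup item that shows an outline when the third-person character can see and reach it.
; When the character begins overlapping ItemModel, it applies M_Outline as an overlay material if the mesh overlaps both the character's SightBox and RangeBox.
; Any end overlap on ItemModel clears the overlay, without checking which actor left.
; The file contains only this highlight logic, with no pickup handling.
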(event `self.ReceiveTick`
  (params (DeltaSeconds :type "Float (single-precision)")))

(event `self.ItemModel.OnComponentBeginOverlap`
  (params (OverlappedComponent :type "PrimitiveComponent Object Reference") (OtherActor :type "Actor Object Reference") (OtherComp :type "PrimitiveComponent Object Reference") (OtherBodyIndex :type Integer) (bFromSweep :type Boolean) (SweepResult :type "HitResult Structure (by ref)"))
  (bind _asbp_third_person_character (cast `/Game/ThirdPerson/Blueprints/BP_ThirdPersonCharacter` OtherActor))
  (if (and (`PrimitiveComponent.IsOverlappingComponent` (`self.ItemModel`) (`/Game/ThirdPerson/Blueprints/BP_ThirdPersonCharacter.Sight Box` _asbp_third_person_character)) (`PrimitiveComponent.IsOverlappingComponent` (`self.ItemModel`) (`/Game/ThirdPerson/Blueprints/BP_ThirdPersonCharacter.Range Box` _asbp_third_person_character)))
    (`MeshComponent.SetOverlayMaterial` (`self.ItemModel`) "/Game/Material/M_Outline.M_Outline")))

(event `self.ItemModel.OnComponentEndOverlap`
  (params (OverlappedComponent :type "PrimitiveComponent Object Reference") (OtherActor :type "Actor Object Reference") (OtherComp :type "PrimitiveComponent Object Reference") (OtherBodyIndex :type Integer))
  (`MeshComponent.SetOverlayMaterial` (`self.ItemModel`) null))

(fn `UserConstructionScript`)
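; Score manager that tracks a running score and stores it per round as the player one or player two score.
; On BeginPlay it binds to every minigame's completion and, inside that same loop, creates a score widget per minigame, keeping only the last reference.
; Completion calls AddScore, scaling a default meal score plus time remaining by meal quality, though both inputs are currently hardcoded.
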(event `self.ReceiveBeginPlay`
  (bind _outactors (`GameplayStatics.GetAllActorsOfClass` "/Game/MiniGames/BP_MiniGameBase.BP_MiniGameBase_C"))
  (for _array_element _outactors
    (add `/Game/MiniGames/BP_MiniGameBase.MinigameCompleted` _array_element (delegate `MinigameCompleted_Event`))
    (bind _returnvalue (`|CreateWidget` "/Game/GameLoopWidgets/WBP_Score.WBP_Score_C"))
    (bind _output_get (set `self.Score Widget` _returnvalue))
    (`UserWidget.AddToViewport` _output_get 0)))

(event `MinigameCompleted_Event`
  (`self.Add Score` 1 1))

(fn `Add Score`
  (params (mealQuality :type Integer) (timeRemaining :type Integer))
  (locals (mealScoreDefault :type Integer :default 100))
  ;[1 1 1] possible score calculation starts with a default meal score and then adjusts it based on the quality of the meal and the time remaining
  (set `self.currentScore` (+ (* mealQuality (+ timeRemaining (`local.mealScoreDefault`))) (`self.currentScore`))))

(fn `AddScoreSimple`
  (params (scoreGained :type Integer))
  (set `self.currentScore` (+ scoreGained (`self.currentScore`))))

(fn `Remove Score Widget`
  (`Widget.RemoveFromParent` (`self.Score Widget`)))

(fn `ResetScore`
  (set `self.currentScore` 0)
  (set `self.p1Score` 0)
  (set `self.p2Score` 0))

(fn `SetScore`
  (params (currentRound :type Integer))
  (bind _currentscore (`self.currentScore`))
  (if (== currentRound 1)
    (set `self.p1Score` _currentscore)
    (elif (== currentRound 2)
      (set `self.p2Score` _currentscore))))

(fn `Test Function`
  (`KismetSystemLibrary.PrintString` "Hello"))

(fn `UserConstructionScript`)
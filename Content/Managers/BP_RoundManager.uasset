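; Round manager for a Rat and Chef game that runs timed rounds and their start and end overlays.
; BeginRound teleports pans and spatulas to hardcoded spots, returns both characters to spawns, resets score, and briefly shows the round number.
; A self-calling Delay event counts down in tenth-second steps.
; At zero, unless DebugMode is set, it shows the end overlay, then sets RoundEnded after a short delay.
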(event `TimerDecrementEvent`
  (`KismetSystemLibrary.Delay` 0.1)
  (bind _output_get (set `self.Counter` (- (`self.Counter`) 0.1)))
  (if (> _output_get 0.0)
    (`self.TimerDecrementEvent`)
    (else
      (`KismetSystemLibrary.PrintString` "Timer Done")
      (if (not (`self.DebugMode`))
        (`self.FinishRound`)))))

(event `BeginRound`
  (params (RoundNum :type Integer))
  (set `self.Round Number` RoundNum)
  (`self.RoundSetup`)
  (`self.RoundUI_Update`)
  (`self.RoundUI_Start`)
  (`KismetSystemLibrary.Delay` 2.0)
  (`self.RoundUI_Fade`)
  (`self.TimerDecrementEvent`))

(event `FinishRound`
  (`self.RoundUi_Finish`)
  (`KismetSystemLibrary.Delay` 2.0)
  (set `self.Round Ended` true))

(fn `Reset Positions`
  (`self.K2_SetActorLocation` (`self.Rat`) (`self.K2_GetActorLocation` (`self.Rat Spawn`)) false false)
  (`self.K2_SetActorLocation` (`self.Chef`) (`self.K2_GetActorLocation` (`self.Chef Spawn `)) false false)
  (`/Game/Managers/BP_ScoreManager.ResetScore` (`self.Score Manager`))
  (`|ExecutionSequence`
    (:`then_0`
      (bind _outactors (`GameplayStatics.GetAllActorsOfClass` "/Game/PickUpable/Blueprints/BP_Pan.BP_Pan_C"))
      (for _array_element _outactors
        (`self.K2_SetActorLocation` _array_element (1040.0 1500.0 100.0) false true)))
    (:`then_1`
      (bind _outactors_2 (`GameplayStatics.GetAllActorsOfClass` "/Game/PickUpable/Blueprints/BP_Spatula.BP_Spatula_C"))
      (for _array_element_2 _outactors_2
        (`self.K2_SetActorLocation` _array_element_2 (690.0 630.0 100.0) false true)))))

(fn `RoundSetup`
  (`self.Reset Positions`)
  (set `self.Counter` (`self.Round Length`))
  (set `self.Round Ended` false))

(fn `RoundUI_Create`
  (bind _returnvalue (`|CreateWidget` "/Game/RoundUI/UI_RoundUI.UI_RoundUI_C"))
  (bind _output_get (set `self.Round UI` _returnvalue))
  (`UserWidget.AddToViewport` _output_get 0))

(fn `RoundUI_Fade`
  (`Widget.SetVisibility` (`self.Round UI`) "Hidden"))

(fn `RoundUi_Finish`
  (bind _round_ui (`self.Round UI`))
  (`Widget.SetVisibility` _round_ui "Visible")
  (`Widget.SetVisibility` (`/Game/RoundUI/UI_RoundUI.Background` _round_ui) "Visible")
  (`Widget.SetVisibility` (`/Game/RoundUI/UI_RoundUI.OverlayRoundStart` _round_ui) "Hidden")
  (`Widget.SetVisibility` (`/Game/RoundUI/UI_RoundUI.OverlayRoundEnd` _round_ui) "Visible"))

(fn `RoundUI_Restart`
  (`Widget.RemoveFromParent` (`self.Round UI`)))

(fn `RoundUI_Start`
  (bind _round_ui (`self.Round UI`))
  (`Widget.SetVisibility` _round_ui "Visible")
  (`Widget.SetVisibility` (`/Game/RoundUI/UI_RoundUI.Background` _round_ui) "Visible")
  (`Widget.SetVisibility` (`/Game/RoundUI/UI_RoundUI.OverlayRoundStart` _round_ui) "Visible")
  (`Widget.SetVisibility` (`/Game/RoundUI/UI_RoundUI.OverlayRoundEnd` _round_ui) "Hidden"))

(fn `RoundUI_Update`
  (set `TextBlock.Text` (`KismetTextLibrary.Conv_StringToText` (`KismetStringLibrary.Concat_StrStr` "Round " (`KismetStringLibrary.Conv_IntToString` (`self.Round Number`)))) (`/Game/RoundUI/UI_RoundUI.RoundNo_Text` (`self.Round UI`))))

(fn `Timer`)

(fn `UserConstructionScript`)
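; Frying minigame Blueprint that only the Chef can start, never the Rat.
; CanStart finds the third-person character and allows play only if its held item has the ingredient tag and is a BP_Ingredient subclass.
; An input prompt starts hidden and is toggled by show and hide events.
; GetActorOwner exposes the owning actor.
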(event `self.ReceiveBeginPlay`
  (`SceneComponent.SetVisibility` (`self.InputPrompt`) false false))

(event `/Game/InputPromptUI/BPI_InputPromptUI.HidePrompt`
  (`SceneComponent.SetVisibility` (`self.InputPrompt`) false false))

(event `/Game/InputPromptUI/BPI_InputPromptUI.DisplayPrompt`
  (`SceneComponent.SetVisibility` (`self.InputPrompt`) true false))

(fn `Can Start`
  (params (IsRat :type Boolean))
  (returns (CanStart :type Boolean))
  (locals (StartGame :type Boolean))
  ;[0.9244 1 0.379] Only Chef can play this minigame
  (if IsRat
    (set `local.StartGame` false :!label _label)
    (else
      (bind _returnvalue (`GameplayStatics.GetActorOfClass` "/Game/ThirdPerson/Blueprints/BP_ThirdPersonCharacter.BP_ThirdPersonCharacter_C"))
      (if (`/Game/ThirdPerson/Blueprints/BP_ThirdPersonCharacter.HasItem` _returnvalue)
        (bind _itemreference (`/Game/ThirdPerson/Blueprints/BP_ThirdPersonCharacter.ItemReference` _returnvalue))
        (if (and (`self.ActorHasTag` _itemreference (`self.IngredientTag`)) (`KismetMathLibrary.ClassIsChildOf` (`GameplayStatics.GetObjectClass` _itemreference) "/Game/Ingredients/BP_Ingredient.BP_Ingredient_C"))
          (set `local.StartGame` true)
          (else
            (goto _label)))
        (else
          (goto _label)))))
  (return (`local.StartGame`)))

(fn `GetActorOwner`
  (returns (ActorName :type String))
  (return (`self.Actor Owner`)))

(fn `UserConstructionScript`
  (`parent.UserConstructionScript`))
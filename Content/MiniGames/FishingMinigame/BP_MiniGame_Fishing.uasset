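; Fishing minigame actor that defines who may start the game: only the Chef, never the Rat.
; Its Can Start check passes only when the BP_ThirdPersonCharacter holds an item derived from BP_Ingredient.
; That character is looked up by class with GetActorOfClass rather than passed in.
; The event graph holds only disabled stubs, so this Blueprint contains no fishing gameplay of its own.
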(fn `Can Start`
  (params (IsRat :type Boolean))
  (returns (CanStart :type Boolean))
  ;[0.9244 1 0.379] Only Chef can play this minigame
  (if IsRat
    (return (not IsRat))
    (else
      (bind _returnvalue (`GameplayStatics.GetActorOfClass` "/Game/ThirdPerson/Blueprints/BP_ThirdPersonCharacter.BP_ThirdPersonCharacter_C"))
      (if (`/Game/ThirdPerson/Blueprints/BP_ThirdPersonCharacter.HasItem` _returnvalue)
        (if (`KismetMathLibrary.ClassIsChildOf` (`GameplayStatics.GetObjectClass` (`/Game/ThirdPerson/Blueprints/BP_ThirdPersonCharacter.ItemReference` _returnvalue)) "/Game/ThirdPerson/Blueprints/BP_Ingredient.BP_Ingredient_C")
          (return (not IsRat)))))))

(fn `UserConstructionScript`
  (`parent.UserConstructionScript`))
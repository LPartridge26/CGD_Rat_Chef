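; BP_MiniGame_Poop is a rat-versus-chef minigame where the rat leaves poop and the chef clears it.
; CanStart admits chefs while broken, and rats while unbroken once WireCooldown, decremented on Tick, runs out.
; ExitMinigame spawns or clears the poop mesh by player role, toggling IsBroken and the linked minigame's IsPlayable.
; The completion check is disconnected, so every exit applies the change.
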(event `self.ReceiveBeginPlay`
  (`parent.ReceiveBeginPlay`))

(event `Clear Poop`
  ;[0.07604 0.07604 0.07604] Removing poop model
  (`StaticMeshComponent.SetStaticMesh` (`self.Wire`) null)
  (set `/Game/MiniGames/BP_MiniGameBase.Is Playable` true (`self.Linked Mini Game`))
  (set `self.IsBroken` false))

(event `self.ReceiveActorBeginOverlap`
  (params (OtherActor :type "Actor Object Reference"))
  (`parent.ReceiveActorBeginOverlap` OtherActor))

(event `Spawn  Poop`
  ;[0.07451 0.07451 0.07451] Adds poop model
  (`StaticMeshComponent.SetStaticMesh` (`self.Wire`) "/Game/MiniGames/RatPoopMiniGame/Models/poop.poop")
  (set `/Game/MiniGames/BP_MiniGameBase.Is Playable` false (`self.Linked Mini Game`))
  (set `self.IsBroken` true))

(event `self.ReceiveTick`
  (params (DeltaSeconds :type "Float (single-precision)"))
  ;[1 1 1] Cooldown for wires
  (set `self.WireCooldown` (- (`self.WireCooldown`) DeltaSeconds)))

(fn `Can Start`
  (params (IsRat :type Boolean))
  (returns (CanStart :type Boolean))
  (if (and (== (`self.IsBroken`) true) (== IsRat false))
    (set `self.StartGame` true)
    (else
      (set `self.StartGame` false)
      (if (and (and IsRat (== (`self.IsBroken`) false)) (<= (`self.WireCooldown`) 0.0))
        (set `self.StartGame` true)
        (else
          (set `self.StartGame` false)))))
  (return (`self.StartGame`)))

(fn `ExitMinigame`
  (params (IsRatPlayer :type Boolean))
  (`parent.ExitMinigame` IsRatPlayer)
  ;[1 1 1] if RAT - break
  ; if CHEF - fix
  (if IsRatPlayer
    (`self.Spawn  Poop`)
    (else
      (`self.Clear Poop`))))

(fn `StartMinigame`
  (params (IsRatPlayer :type Boolean) (OwningPlayer :type "PlayerController Object Reference"))
  (`parent.StartMinigame` IsRatPlayer OwningPlayer))

(fn `UserConstructionScript`
  (`parent.UserConstructionScript`))
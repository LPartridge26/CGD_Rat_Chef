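; Base actor for score-driven minigames played by a Rat or Chef player, with CanStart returning true by default.
; StartMinigame adds the minigame widget and a role-specific progress bar to the owning player's screen, and ExitMinigame removes both and resets the score.
; Tap, hold and cancel inputs forward to the minigame widget.
; AddScore updates the bar and, at max score, signals completion through the widget and plays a coin sound.
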(fn `AddScore`
  (params (ScoreToAdd :type "Float (double-precision)"))
  (bind _returnvalue (+ (`self.CurrentScore`) ScoreToAdd))
  (bind _returnvalue_2 (/ (`self.CurrentScore`) (`self.MaxScore`)))
  (if (> _returnvalue 0.0)
    (set `self.CurrentScore` _returnvalue)
    (message `/Game/MiniGameInteractiveControls/BPI_ProgressBar.UpdateBar` (`self.ProgressBarWidget`) _returnvalue_2)
    (if (>= _returnvalue_2 1.0)
      (`self.MinigameCompleted` (`self.MinigameBaseUI`))
      (`KismetSystemLibrary.PrintString` "Hello")
      (`GameplayStatics.PlaySound2D` "/Game/Interface_And_Item_Sounds/WAV/Coins_13.Coins_13" 4.0 1.0 0.0 null null))))

(fn `Can Start`
  (params (IsRat :type Boolean))
  (returns (CanStart :type Boolean))
  (return true))

(fn `CancelledInput`
  (params (IsRat :type Boolean))
  (bind _minigamebaseui (`self.MinigameBaseUI`)
    (:`then`
      (`/Game/MiniGames/UI_MiniGameBase.CancelledInput` _minigamebaseui IsRat))
    (:`else`)))

(fn `ExitMinigame`
  (params (IsRatPlayer :type Boolean))
  (`Widget.RemoveFromParent` (`self.MinigameBaseUI`))
  (`Widget.RemoveFromParent` (`self.ProgressBarWidget`))
  (set `self.CurrentScore` 0.0))

(fn `Get Current Score`
  (returns (`Current Score` :type "Float (double-precision)"))
  (return (`self.CurrentScore`)))

(fn `HoldInput`
  (params (TimeHeld :type "Float (double-precision)") (IsRat :type Boolean))
  (bind _minigamebaseui (`self.MinigameBaseUI`)
    (:`then`
      (`/Game/MiniGames/UI_MiniGameBase.HoldInput` _minigamebaseui TimeHeld IsRat))
    (:`else`)))

(fn `IsComplete`
  (returns (IsComplete :type Boolean))
  (return (>= (`self.CurrentScore`) (`self.MaxScore`))))

(fn `StartMinigame`
  (params (IsRatPlayer :type Boolean) (OwningPlayer :type "PlayerController Object Reference"))
  (bind _output_get (set `self.Is Rat Player` IsRatPlayer))
  (bind _returnvalue (`|CreateWidget` (`self.MinigameWidget`) OwningPlayer))
  (bind _asui_mini_game_base (cast `/Game/MiniGames/UI_MiniGameBase` _returnvalue))
  (bind _output_get_2 (set `self.MinigameBaseUI` _asui_mini_game_base))
  (set `/Game/MiniGames/UI_MiniGameBase.IsRatPlayer` _output_get _asui_mini_game_base)
  (set `/Game/MiniGames/UI_MiniGameBase.BaseMinigameRef` self _output_get_2)
  (`UserWidget.AddToPlayerScreen` (`self.MinigameBaseUI`) 0)
  (bind _returnvalue_2 (`|CreateWidget` (select `bool` IsRatPlayer :`false` "/Game/MiniGameInteractiveControls/UI_Chef_ProgressBar.UI_Chef_ProgressBar_C" :`true` "/Game/MiniGameInteractiveControls/UI_Rat_ProgressBar.UI_Rat_ProgressBar_C" :!type "UserWidget Class Reference") OwningPlayer))
  (`UserWidget.AddToPlayerScreen` _returnvalue_2 0)
  (set `self.ProgressBarWidget` _returnvalue_2))

(fn `TapInput`
  (params (IsRat :type Boolean))
  (bind _minigamebaseui (`self.MinigameBaseUI`)
    (:`then`
      (`/Game/MiniGames/UI_MiniGameBase.TapInput` _minigamebaseui IsRat))
    (:`else`)))

(fn `UpdateScore`)

(fn `UserConstructionScript`)
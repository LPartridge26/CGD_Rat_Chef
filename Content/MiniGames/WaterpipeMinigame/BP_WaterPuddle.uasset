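; BP_WaterPuddle is a puddle actor for the waterpipe minigame that slows the player character.
; Overlap begin and end events switch BP_ThirdPersonCharacter's max walk speed between fixed slow and faster values, without checking puddle visibility.
; SpawnPuddle makes the Puddle component visible and prints a debug message.
; DrainPuddle only prints a message and does not yet hide the puddle.
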(event `self.ReceiveActorBeginOverlap`
  (params (OtherActor :type "Actor Object Reference"))
  (bind _asbp_third_person_character (cast `/Game/ThirdPerson/Blueprints/BP_ThirdPersonCharacter` OtherActor))
  (set `CharacterMovementComponent.MaxWalkSpeed` 100.0 (`Character.CharacterMovement` _asbp_third_person_character)))

(event `self.ReceiveActorEndOverlap`
  (params (OtherActor :type "Actor Object Reference"))
  (bind _asbp_third_person_character (cast `/Game/ThirdPerson/Blueprints/BP_ThirdPersonCharacter` OtherActor))
  (set `CharacterMovementComponent.MaxWalkSpeed` 300.0 (`Character.CharacterMovement` _asbp_third_person_character)))

(event `SpawnPuddle`
  (`KismetSystemLibrary.PrintString` "Creating Puddles")
  (`SceneComponent.SetVisibility` (`self.Puddle`) true false))

(event `DrainPuddle`
  (`KismetSystemLibrary.PrintString` "Draining Puddles"))

(fn `UserConstructionScript`)
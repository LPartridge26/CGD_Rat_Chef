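; BP_MiniGame_Pipes is the waterpipe minigame Blueprint, playable by both rat and chef players.
; Can Start lets a chef play only while the pipe is leaking and a rat only while it is not.
; StartMinigame creates the pipes UI with a randomly picked puddle, registers itself on it as a UI_MiniGameBase, and adds a rat or chef progress bar to the player screen.
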(fn `Can Start`
  (params (IsRat :type Boolean))
  (returns (CanStart :type Boolean))
  (if (and (== (`self.IsLeaking`) true) (== IsRat false))
    (set `self.StartGame` true)
    (else
      (set `self.StartGame` false)
      (if (and IsRat (== (`self.IsLeaking`) false))
        (set `self.StartGame` true)
        (else
          (set `self.StartGame` false)))))
  (return (`self.StartGame`)))

(fn `StartMinigame`
  (params (IsRatPlayer :type Boolean) (OwningPlayer :type "PlayerController Object Reference"))
  (bind _puddle (`self.Puddle`))
  (bind _output_get (set `self.Is Rat Player` IsRatPlayer))
  (bind _returnvalue (`|CreateWidget` "/Game/MiniGames/WaterpipeMinigame/UI_MiniGame_Pipes.UI_MiniGame_Pipes_C" OwningPlayer (`|GetArrayItem` _puddle (`KismetMathLibrary.RandomInteger` (`KismetArrayLibrary.Array_Length` _puddle))) null IsRatPlayer))
  (bind _asui_mini_game_base (cast `/Game/MiniGames/UI_MiniGameBase` _returnvalue))
  (bind _output_get_2 (set `self.MinigameBaseUI` _asui_mini_game_base))
  (set `/Game/MiniGames/UI_MiniGameBase.IsRatPlayer` _output_get _asui_mini_game_base)
  (set `/Game/MiniGames/UI_MiniGameBase.BaseMinigameRef` self _output_get_2)
  (`UserWidget.AddToPlayerScreen` (`self.MinigameBaseUI`) 0)
  (bind _returnvalue_2 (`|CreateWidget` (select `bool` IsRatPlayer :`false` "/Game/MiniGameInteractiveControls/UI_Chef_ProgressBar.UI_Chef_ProgressBar_C" :`true` "/Game/MiniGameInteractiveControls/UI_Rat_ProgressBar.UI_Rat_ProgressBar_C" :!type "UserWidget Class Reference")))
  (`UserWidget.AddToPlayerScreen` _returnvalue_2 0)
  (set `self.ProgressBarWidget` _returnvalue_2))

(fn `UserConstructionScript`
  (`parent.UserConstructionScript`))
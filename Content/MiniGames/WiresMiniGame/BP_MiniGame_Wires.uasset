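; BP_MiniGame_Wires is a child minigame for a set of wires that rats can break and non-rat players (chefs) can fix.
; BreakWires and FixWires swap the mesh, add or remove a Niagara spark effect, and toggle whether the linked minigame is playable.
; CanStart admits non-rats only when broken, and rats only when intact and the Tick-decremented cooldown has expired.
; The role branch in ExitMinigame is empty.
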(event `self.ReceiveBeginPlay`
  (`parent.ReceiveBeginPlay`)
  (`ActorComponent.K2_DestroyComponent` (`self.GuideMarker`)))

(event `FixWires`
  ;[0.07604 0.07604 0.07604] Change wires to appear fixed
  (`StaticMeshComponent.SetStaticMesh` (`self.Wire`) "/Game/MiniGames/WiresMiniGame/Models/wires.wires")
  (set `/Game/MiniGames/BP_MiniGameBase.Is Playable` true (`self.Linked Mini Game`))
  (set `self.IsBroken` false)
  (if (`KismetSystemLibrary.IsValid` (`self.Spark Effectt Reference`))
    (`ActorComponent.K2_DestroyComponent` (`self.Spark Effectt Reference`))))

(event `self.ReceiveActorBeginOverlap`
  (params (OtherActor :type "Actor Object Reference"))
  (`parent.ReceiveActorBeginOverlap` OtherActor))

(event `BreakWires`
  ;[0.07451 0.07451 0.07451] Change wires to appear broken
  (`StaticMeshComponent.SetStaticMesh` (`self.Wire`) "/Game/MiniGames/WiresMiniGame/Models/wires_broken.wires_broken")
  (set `/Game/MiniGames/BP_MiniGameBase.Is Playable` false (`self.Linked Mini Game`))
  (set `self.IsBroken` true)
  (if (not (`KismetSystemLibrary.IsValid` (`self.Spark Effectt Reference`)))
    (bind _returnvalue (`NiagaraFunctionLibrary.SpawnSystemAttached` "/Game/MiniGames/WiresMiniGame/Effects/FX_Sparks.FX_Sparks" (`self.Wire`) "None" (0.0 0.0 0.0) (struct) "KeepRelativeOffset"))
    (bind _output_get (set `self.Spark Effectt Reference` _returnvalue))
    (`SceneComponent.SetRelativeScale3D` _output_get (4.0 4.0 4.0))
    (`SceneComponent.K2_SetRelativeLocation` _output_get (0.0 0.0 0.1) false false)))

(event `self.ReceiveTick`
  (params (DeltaSeconds :type "Float (single-precision)"))
  ;[1 1 1] Cooldown for wires
  (set `self.WireCooldown` (- (`self.WireCooldown`) DeltaSeconds)))

(fn `Can Start`
  (params (IsRat :type Boolean))
  (returns (CanStart :type Boolean))
  (if (and (== (`self.IsBroken`) true) (== IsRat false))
    (set `self.StartGame` true)
    (else
      (set `self.StartGame` false)
      (if (and (and IsRat (== (`self.IsBroken`) false)) (<= (`self.WireCooldown`) 0.0))
        (set `self.StartGame` true)
        (else
          (set `self.StartGame` false)))))
  (return (`self.StartGame`)))

(fn `ExitMinigame`
  (params (IsRatPlayer :type Boolean))
  (`parent.ExitMinigame` IsRatPlayer)
  ;[1 1 1] if RAT - break
  ; if CHEF - fix
  (if IsRatPlayer
    _))

(fn `GetMarkerType`
  (returns (MarkerType :type String))
  (return ""))

(fn `StartMinigame`
  (params (IsRatPlayer :type Boolean) (OwningPlayer :type "PlayerController Object Reference"))
  (`parent.StartMinigame` IsRatPlayer OwningPlayer))

(fn `UserConstructionScript`
  (`parent.UserConstructionScript`))
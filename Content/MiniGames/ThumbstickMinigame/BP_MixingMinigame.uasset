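; Mixing station minigame that only the Chef, not the Rat, can start, and only while holding an ingredient.
; CanStart checks the third-person character's held item against BP_Ingredient, overriding a parent minigame class along with the marker and prompt type getters.
; Tick repeats that held-item check to swap the mesh to a highlight material.
; BeginPlay destroys the GuideMarker and InputPrompt components.
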(event `self.ReceiveTick`
  (params (DeltaSeconds :type "Float (single-precision)"))
  (bind _staticmesh (`self.StaticMesh`))
  (bind _returnvalue (`GameplayStatics.GetActorOfClass` "/Game/ThirdPerson/Blueprints/BP_ThirdPersonCharacter.BP_ThirdPersonCharacter_C"))
  (if (`/Game/ThirdPerson/Blueprints/BP_ThirdPersonCharacter.HasItem` _returnvalue)
    (if (`KismetMathLibrary.ClassIsChildOf` (`GameplayStatics.GetObjectClass` (`/Game/ThirdPerson/Blueprints/BP_ThirdPersonCharacter.ItemReference` _returnvalue)) "/Game/Ingredients/BP_Ingredient.BP_Ingredient_C")
      (`PrimitiveComponent.SetMaterial` _staticmesh 0 "/Game/Material/M_Mixing_Highlight.M_Mixing_Highlight")
      (else
        (`PrimitiveComponent.SetMaterial` _staticmesh 0 "/Game/LevelPrototyping/AssetPacks/KayKit_Restaurant_Bits/fbx/restaurant.restaurant" :!label _label)))
    (else
      (goto _label))))

(event `self.ReceiveBeginPlay`
  (`ActorComponent.K2_DestroyComponent` (`self.GuideMarker`))
  (`ActorComponent.K2_DestroyComponent` (`self.InputPrompt`)))

(fn `Can Start`
  (params (IsRat :type Boolean))
  (returns (CanStart :type Boolean))
  ;[0.9244 1 0.379] Only Chef can play this minigame
  (if IsRat
    (set `self.StartGame` false :!label _label)
    (return (`self.StartGame`))
    (else
      (bind _returnvalue (`GameplayStatics.GetActorOfClass` "/Game/ThirdPerson/Blueprints/BP_ThirdPersonCharacter.BP_ThirdPersonCharacter_C"))
      (if (`/Game/ThirdPerson/Blueprints/BP_ThirdPersonCharacter.HasItem` _returnvalue)
        (if (`KismetMathLibrary.ClassIsChildOf` (`GameplayStatics.GetObjectClass` (`/Game/ThirdPerson/Blueprints/BP_ThirdPersonCharacter.ItemReference` _returnvalue)) "/Game/Ingredients/BP_Ingredient.BP_Ingredient_C")
          (set `self.StartGame` true)
          (return (`self.StartGame`)))
        (else
          (goto _label))))))

(fn `GetMarkerType`
  (returns (MarkerType :type String))
  (return (`self.ObjectType`)))

(fn `GetPromptType`
  (returns (PromptType :type String))
  (return (`self.ObjectType`)))

(fn `UserConstructionScript`
  (`parent.UserConstructionScript`))
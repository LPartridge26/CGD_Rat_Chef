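; Fishing minigame station Blueprint that only the Chef, not the Rat, can start, and only while holding an ingredient.
; CanStart looks up the third-person character and checks that its held item derives from BP_Ingredient.
; An input prompt and guide marker start hidden and toggle through show/hide events, with getters exposing marker type and owning actor.
; The file contains no fishing gameplay, and its bubbling-sound nodes are disconnected.
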(event `self.ReceiveBeginPlay`
  (`SceneComponent.SetVisibility` (`self.InputPrompt`) false false)
  (`SceneComponent.SetVisibility` (`self.GuideMarker`) false false))

(event `/Game/UI/InputPromptUI/BPI_InputPromptHolder.HidePrompt`
  (`SceneComponent.SetVisibility` (`self.InputPrompt`) false false))

(event `/Game/UI/InputPromptUI/BPI_InputPromptHolder.DisplayPrompt`
  (`SceneComponent.SetVisibility` (`self.InputPrompt`) true false))

(event `/Game/UI/GuideMarkerGUI/BPI_GuideMarkerHolder.HideMarker`
  (`SceneComponent.SetVisibility` (`self.GuideMarker`) false false))

(event `/Game/UI/GuideMarkerGUI/BPI_GuideMarkerHolder.DisplayMarker`
  (`SceneComponent.SetVisibility` (`self.GuideMarker`) true false))

(fn `Can Start`
  (params (IsRat :type Boolean))
  (returns (CanStart :type Boolean))
  ;[0.9244 1 0.379] Only Chef can play this minigame
  (if (not IsRat)
    (bind _returnvalue (`GameplayStatics.GetActorOfClass` "/Game/ThirdPerson/Blueprints/BP_ThirdPersonCharacter.BP_ThirdPersonCharacter_C"))
    (if (`/Game/ThirdPerson/Blueprints/BP_ThirdPersonCharacter.HasItem` _returnvalue)
      (if (`KismetMathLibrary.ClassIsChildOf` (`GameplayStatics.GetObjectClass` (`/Game/ThirdPerson/Blueprints/BP_ThirdPersonCharacter.ItemReference` _returnvalue)) "/Game/Ingredients/BP_Ingredient.BP_Ingredient_C")
        (set `self.StartGame` true)
        (else
          (set `self.StartGame` false :!label _label)))
      (else
        (goto _label)))
    (return (`self.StartGame`))))

(fn `GetMarkerType`
  (returns (MarkerType :type String))
  (return (`self.MarkerType`)))

(fn `InputPrompt_GetActorOwner`
  (returns (ActorName :type String))
  (return (`self.Actor Owner`)))

(fn `Marker_GetActorOwner`
  (returns (ActorName :type String))
  (return (`self.Actor Owner`)))

(fn `UserConstructionScript`
  (`parent.UserConstructionScript`))